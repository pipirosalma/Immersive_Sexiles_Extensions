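; Actor component for extra character states in a capture-style mechanic: knockout, poisoning, waking, surrender and bound poses.
; Knockout and poison events set Unconscious, wait a fixed delay ignoring UnconDuration, then restore Passive and remove the debuff; their montages are disconnected.
; Pose events play or stop montages, and a relocation event chains through SRV and C events to move and rotate an actor.
; Helpers resolve the owning character, sphere-trace nearby pawns and track captured/collared flags.
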(event Custom|setlocation_C
  (params (TeleportActor :type Base%20Player%20Char%20Object%20Reference) (TeleportLocation :type Vector) (TeleportRotation :type Rotator))
  (Transformation|SetActorLocation TeleportActor TeleportLocation false false)
  (Class|Actor|AddActorWorldRotation TeleportActor TeleportRotation))

(event Custom|ClearKneeling
  (params (CharRef :type Character%20Object%20Reference))
  (Animation|StopAnimMontage CharRef "/Game/Characters/humans/animations/emotes/AM_emote_kneeling.AM_emote_kneeling"))

(event Custom|BoundGround
  (params (Char%20Ref :type Character%20Object%20Reference))
  (Animation|PlayAnimMontage Char%20Ref "/Game/Mods/Immersive_Sexiles_Extensions/Assets/Animation/AM_emote_bound_sleeping_ground.AM_emote_bound_sleeping_ground" 1.0 "None"))

(event Custom|setlocation_SRV
  (params (TeleportActor :type Base%20Player%20Char%20Object%20Reference) (TeleportLocation :type Vector) (TeleportRotation :type Rotator))
  (CallFunction|SetlocationC TeleportActor TeleportLocation TeleportRotation))

(event Custom|Surrender
  (params (CharRef :type Character%20Object%20Reference))
  (Animation|PlayAnimMontage CharRef "/Game/Characters/humans/animations/emotes/AM_emote_kneeling.AM_emote_kneeling" 1.0 "None"))

(event Custom|PlayPoisonedAnimation
  (params (CharacterReference :type Character%20Object%20Reference) (Base%20Player%20Char :type Base%20Player%20Char%20Object%20Reference) (UnconDuration :type Float%20%28single-precision%29))
  (Default|UpdateCharacterState Base%20Player%20Char "Unconscious")
  (Utilities|FlowControl|Delay 6e+01)
  (Default|UpdateCharacterState Base%20Player%20Char "Passive")
  (Default|HandleCombatState Base%20Player%20Char)
  (Class|BasePlayerCharInterface|UpdateCharacterState(Message) Base%20Player%20Char "Passive")
  (Default|ClearSubstates Base%20Player%20Char)
  (Default|RemoveBuff (Variables|/Game/Characters/BaseBPCombat.BaseBPCombat_C|Get00_BP_AC_BuffSystem Base%20Player%20Char) "/Game/Mods/Immersive_Sexiles_Extensions/System/BP_AC_Debuff_Unconscious_State.BP_AC_Debuff_Unconscious_State_C")
  (Default|HandleCombatState Base%20Player%20Char))

(event Custom|PlayKnockoutAnimation
  (params (Character%20Reference :type Character%20Object%20Reference) (BPCharacter%20Reference :type Base%20Player%20Char%20Object%20Reference) (Uncon%20Duration :type Float%20%28single-precision%29))
  (Default|UpdateCharacterState BPCharacter%20Reference "Unconscious")
  (Utilities|FlowControl|Delay 6e+01)
  (Default|UpdateCharacterState BPCharacter%20Reference "Passive")
  (Default|HandleCombatState BPCharacter%20Reference)
  (Class|BasePlayerCharInterface|UpdateCharacterState(Message) BPCharacter%20Reference "Passive")
  (Default|ClearSubstates BPCharacter%20Reference)
  (Default|RemoveBuff (Variables|/Game/Characters/BaseBPCombat.BaseBPCombat_C|Get00_BP_AC_BuffSystem BPCharacter%20Reference) "/Game/Mods/Immersive_Sexiles_Extensions/System/BP_AC_Debuff_Knockout_State.BP_AC_Debuff_Knockout_State_C")
  (Default|HandleCombatState BPCharacter%20Reference))

(event Custom|BoundBack
  (params (Char%20Ref :type Character%20Object%20Reference))
  (Animation|PlayAnimMontage Char%20Ref "/Game/Mods/Immersive_Sexiles_Extensions/Assets/Animation/AM_Behind_Back_Bound.AM_Behind_Back_Bound" 1.0 "None"))

(event Custom|WakeUp
  (params (BPChar%20Ref :type Base%20Player%20Char%20Object%20Reference))
  (Default|UpdateCharacterState BPChar%20Ref "Passive")
  (Default|HandleCombatState BPChar%20Ref)
  (Class|BasePlayerCharInterface|UpdateCharacterState(Message) BPChar%20Ref "Passive")
  (Default|ClearSubstates BPChar%20Ref))

(event Custom|setlocation
  (params (TeleportActor :type Base%20Player%20Char%20Object%20Reference) (TeleportLocation :type Vector) (TeleportRotation :type Rotator))
  (CallFunction|SetlocationSRV TeleportActor TeleportLocation TeleportRotation))

(event Custom|BoundKneel
  (params (Char%20Ref :type Character%20Object%20Reference))
  (Animation|PlayAnimMontage Char%20Ref "/Game/Mods/Immersive_Sexiles_Extensions/Assets/Animation/AM_emote_bound_kneeling.AM_emote_bound_kneeling" 1.0 "None"))

(event EventBeginPlay)

(event EventTick
  (params (DeltaSeconds :type Float%20%28single-precision%29)))

(fn GetBasePlayerChar
  (bind _returnvalue (Components|GetOwner))
  (bind _asfun_combat_player_controller (Utilities|Casting|CastToFunCombat_PlayerController _returnvalue)
    (:then
      (bind _asbase_player_char (Utilities|Casting|CastToBasePlayerChar (Pawn|GetControlledPawn _asfun_combat_player_controller))
        (:then
          _)
        (:CastFailed
          _)))
    (:CastFailed
      (bind _asbase_player_char_2 (Utilities|Casting|CastToBasePlayerChar _returnvalue)
        (:then
          (return _asbase_player_char_2))
        (:CastFailed
          _))))
  (return _asbase_player_char))

(fn PointTargetCheck
  (bind _baseplayerchar (CallFunction|GetBasePlayerChar))
  (bind _capsulecomponent (Variables|/Script/Engine.Character|GetCapsuleComponent _baseplayerchar))
  (bind _returnvalue (Transformation|GetWorldLocation _capsulecomponent))
  (bind (_x _y _z) (Math|Vector|BreakVector _returnvalue))
  (bind _aspawn (Utilities|Casting|CastToPawn (Components|GetOwner))
    (:then
      (bind _output_get (Variables|Default|SetLocalTraceStartLocation _returnvalue))
      (bind _output_get_2 (Variables|Default|SetLocalTraceStartLocation (Math|Vector|MakeVector _x _y _z)))
      (bind _outhit (Collision|SphereTraceForObjects _output_get _output_get_2 1.3e+02 (Utilities|Array|MakeArray "ObjectTypeQuery3") false (Utilities|Array|MakeArray _aspawn) "ForDuration"))
      (return (.HitActor (Collision|BreakHitResult _outhit))))
    (:CastFailed
      (return 0))))

(fn AskCollarState
  (bind _baseplayerchar (CallFunction|GetBasePlayerChar))
  (Utilities|Casting|CastToFunCombat_PlayerController (Pawn|GetController _baseplayerchar)
    (:then
      _)
    (:CastFailed
      _))
  (Development|PrintString (Class|ConanPlayerController|GetCharacterName (Variables|/Game/Characters/BasePlayerChar.BasePlayerChar_C|GetPlayerController _baseplayerchar)))
  (return (Variables|Default|GetIsCollared)))

(fn SetCapturedState
  (params (CapturedState :type Boolean))
  (Variables|Default|SetIsCaptured CapturedState))