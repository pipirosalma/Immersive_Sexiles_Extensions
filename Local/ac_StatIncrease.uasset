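; Actor component that appears meant to raise a player stat by a given amount, with helpers to reach the BasePlayerChar through its owning FunCombat_PlayerController.
; SelectAttribute maps the stat name to its current value and returns that level's point cost.
; A loop is built to credit that cost as undistributed points and call GiveAttribute once per increase.
; The StatIncrease entry is not wired to this loop, so it currently does nothing.
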(fn GetBasePlayerChar
  (bind _asfun_combat_player_controller (Utilities|Casting|CastToFunCombat_PlayerController (Components|GetOwner))
    (:then
      (bind _asbase_player_char (Utilities|Casting|CastToBasePlayerChar (Pawn|GetControlledPawn _asfun_combat_player_controller))
        (:then
          _)
        (:CastFailed
          _)))
    (:CastFailed
      _))
  (return _asbase_player_char))

(fn SelectAttribute
  (switch Utilities|FlowControl|Switch|SwitchonEAttributeType (Variables|Default|GetStatnName)
    (:Health
      (bind _health (CallFunction|GetAttributeHealth "Full"))
      (return (CallFunction|GetAttributePointCost _health)))
    (:Stamina
      (bind _stamina (CallFunction|GetAttributeStamina "Full"))
      (return (CallFunction|GetAttributePointCost _stamina)))
    (:Encumbrance
      (bind _encumbrance (CallFunction|GetAttributeEncumbrance "Full"))
      (return (CallFunction|GetAttributePointCost _encumbrance)))
    (:Might
      (bind _might (CallFunction|GetAttributeMight "Full"))
      (return (CallFunction|GetAttributePointCost _might)))
    (:Accuracy
      (bind _accuracy (CallFunction|GetAttributeAccuracy "Full"))
      (return (CallFunction|GetAttributePointCost _accuracy)))
    (:Athleticism
      (bind _athleticism (CallFunction|GetAttributeAthleticism "Full"))
      (return (CallFunction|GetAttributePointCost _athleticism)))
    (:Metabolism
      (bind _metabolism (CallFunction|GetAttributeMetabolism "Full"))
      (return (CallFunction|GetAttributePointCost _metabolism)))
    (:Resilience
      (bind _resilience (CallFunction|GetAttributeRecilience "Full"))
      (return (CallFunction|GetAttributePointCost _resilience)))))

(fn StatIncrease
  (params (Stat :type EAttributeType%20Enum) (Amount :type Integer))
  ;[1 1 1] Accu
)