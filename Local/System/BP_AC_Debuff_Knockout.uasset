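; Buff component for a knockout debuff that can tip a badly hurt player character into a knockout state.
; Each buff tick it removes itself from NPCs; for players it checks for low health, that they are not already unconscious, and a random roll resisted by Metabolism.
; When all checks pass, it ends itself and adds the Knockout_State buff through the character's buff system, passing along the damage causer.
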(event EventGameplayEffecttoApplyonBuffTick
  (bind _asbase_player_char (Utilities|Casting|CastToBasePlayerChar (Variables|Default|GetOwningCharacter)))
  (bind _isnpc (Default|CheckIsNPC _asbase_player_char))
  (if _isnpc
    (Default|EndBuff (Variables|/Game/Characters/BaseBPCombat.BaseBPCombat_C|Get00_BP_AC_BuffSystem _asbase_player_char) "BP_AC_Debuff_Knockout_C")
    (elif (Math|Boolean|ANDBoolean (>= 0.2 (/ (Math|Conversions|ToFloat(Integer) (Class|ConanCharacter|GetIntStat _asbase_player_char "HealthCurrent" "Full")) (Math|Conversions|ToFloat(Integer) (Default|GetHealthMax _asbase_player_char)))) (Utilities|Enum|NotEqual(Enum) (Class|ConanCharacter|GetCharacterState _asbase_player_char) "Unconscious") (>= (Math|Random|RandomFloatinRange 0.0 1e+02) (/ (Math|Conversions|ToFloat(Integer) (Class|ConanCharacter|GetIntStat _asbase_player_char "AttributeMetabolism" "Full")) 3.0)))
      (Default|EndBuff (Variables|/Game/Characters/BaseBPCombat.BaseBPCombat_C|Get00_BP_AC_BuffSystem _asbase_player_char) "BP_AC_Debuff_Knockout_C")
      (Default|AddBuff (Variables|/Game/Characters/BaseBPCombat.BaseBPCombat_C|Get00_BP_AC_BuffSystem _asbase_player_char) "/Game/Mods/Immersive_Sexiles_Extensions/System/BP_AC_Debuff_Knockout_State.BP_AC_Debuff_Knockout_State_C" (Variables|Default|GetDamageCauser) 0 (Pawn|GetController (Variables|/Script/Engine.Actor|GetInstigator (Variables|Default|GetOwningCharacter)))))))