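; Second horn checkpoint interactable for The Gauntlet quest, which players must activate in sequence.
; On activation it reads CheckPointCount from the player controller's Funcom_PC_Extension component and advances it from 1 to 2.
; Success shows a "Horn Blown" notification and calls BPBSCMulticastSound's InteractableActivate.
; Any other count only shows a "Missing Horn" notification with the count plus one.
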(event EventInteractableActivate
  (params (Component :type Primitive%20Component%20Object%20Reference) (Instigator :type Player%20Controller%20Object%20Reference) (HitIndex :type Integer))
  (bind _asfun_combat_player_controller (Utilities|Casting|CastToFunCombat_PlayerController Instigator))
  (if (> (Utilities|Array|Length (Actor|GetComponentsByClass _asfun_combat_player_controller "/Game/Mods/Immersive_Sexiles_Extensions/Funcom_PC_Extension.Funcom_PC_Extension_C")) 0)
    (if (== (Variables|/Game/Mods/Immersive_Sexiles_Extensions/Funcom_PC_Extension.Funcom_PC_Extension_C|GetCheckPointCount (Utilities|Array|Get(acopy) (Actor|GetComponentsByClass _asfun_combat_player_controller "/Game/Mods/Immersive_Sexiles_Extensions/Funcom_PC_Extension.Funcom_PC_Extension_C"))) 1)
      (bind _output_get (Variables|/Game/Mods/Immersive_Sexiles_Extensions/Funcom_PC_Extension.Funcom_PC_Extension_C|SetCheckPointCount (Utilities|Array|Get(acopy) (Actor|GetComponentsByClass _asfun_combat_player_controller "/Game/Mods/Immersive_Sexiles_Extensions/Funcom_PC_Extension.Funcom_PC_Extension_C")) 2))
      (Default|NotificationText _asfun_combat_player_controller (Utilities|Text|ToText(String) (Utilities|String|Append (Utilities|String|ToString(Text) (Utilities|Text|MakeLiteralText "Horn Blown:")) (Utilities|String|ToString(Integer) _output_get))) false)
      (Default|InteractableActivate (Variables|Default|GetBP_BSC_MulticastSound) Component Instigator HitIndex)
      (else
        (Default|NotificationText _asfun_combat_player_controller (Utilities|Text|ToText(String) (Utilities|String|Append (Utilities|String|ToString(Text) (Utilities|Text|MakeLiteralText "Missing Horn: ")) (Utilities|String|ToString(Integer) (+ (Variables|/Game/Mods/Immersive_Sexiles_Extensions/Funcom_PC_Extension.Funcom_PC_Extension_C|GetCheckPointCount (Utilities|Array|Get(acopy) (Actor|GetComponentsByClass _asfun_combat_player_controller "/Game/Mods/Immersive_Sexiles_Extensions/Funcom_PC_Extension.Funcom_PC_Extension_C"))) 1)))) false)))))

(fn ConstructionScript
  (|CallParentFunction))