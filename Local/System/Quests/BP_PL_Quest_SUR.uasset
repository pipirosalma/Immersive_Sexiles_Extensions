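; Interactable Conan Exiles quest placeable, a drunken pirate's stand that trades putrid meat for a hangover-cure reward.
; On interaction, admins get the parent behavior, while other players get a backpack check leading to Quest1Complete or a descriptive hint message.
; Completion deletes the required items, then adds the reward and shows story text, or notifies an error.
; A second White Rhino Soup quest remains but is unreachable behind a hard-coded false condition.
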(event EventBeginPlay
  (Default|TurnonAll (Variables|Default|GetBP_BAC_TurnLightOnOff))
  (|CallParentFunction))

(event Collision|EventActorBeginOverlap
  (params (OtherActor :type Actor%20Object%20Reference)))

(event EventTick
  (params (DeltaSeconds :type Float%20%28single-precision%29)))

(event EventInteractableActivate
  (params (Component :type Primitive%20Component%20Object%20Reference) (Instigator :type Player%20Controller%20Object%20Reference) (HitIndex :type Integer))
  (bind _output_get (Variables|Default|SetInvestigator Instigator))
  (bind _asconan_player_controller (Utilities|Casting|CastToConanPlayerController _output_get))
  (if (Class|ConanPlayerController|IsAdmin _asconan_player_controller)
    (|CallParentFunction Component Instigator HitIndex)
    (else
      (bind _asconan_character (Utilities|Casting|CastToConanCharacter (Pawn|GetControlledPawn Instigator))
        (:then
          (bind _output_get_2 (Variables|Default|SetConChar _asconan_character))
          (bind _returnvalue (Class|ConanCharacter|GetBackpackInventory _output_get_2))
          (bind _output_get_3 (Variables|Default|SetPlayerInvRef _returnvalue))
          ;[1 1 1] Q1 Requirements
          (Utilities|And+Branch (Class|ItemInventory|HasItembyTemplateID _output_get_3 (Variables|Default|GetQ1_R_ID) (Variables|Default|GetQ1%20R%20Q)) true ; Quest1 Item Check
            (:True
              (CallFunction|Quest1Complete))
            (:False
              ;[1 1 1] Q2 Requirements
              (Utilities|And+Branch false false ; Quest2 Item Check
                (:True
                  (CallFunction|Quest2Complete))
                (:False
                  (Class|ConanCharacter|ClientShowMessage (Variables|Default|GetConChar) (Utilities|Text|MakeLiteralText "Drunken Sot") (Utilities|Text|MakeLiteralText "A man dressed as a pirate and far from the camps of the Black Hand snores atop the stand here.  The smell of ale can be scented from ten yards off, and the brand on his arm marks his as a traitor to the hand.  Fallen flagons and an empty keg mark how he passed the night, and as you approach, his eyes flutter open.

A sign hangs off the stand.  “Cura para la resaca.”  The Zingaran is crudely written, and beneath it is the cost.  A half ton of rotted meat, and five hundred silver.  The five hundred is crossed out, and replaced with two hundred and fifty.  The two hundred fifty is also crossed out, and ‘One hundred’ is scrawled, near illegibly.  The man eyes you for a moment, and then closes his eyes again.

((1000 Putrid Meat))
") :!pinned true) ; Both Quest Requ is missing
                )))))
        (:CastFailed
          (Development|PrintString "Casto to Conan Character Failed"))))))

(fn ConstructionScript
  (|CallParentFunction))

(fn GetArtisanThrallInventory
  (return (Variables|Default|GetThrallInventory)))

(fn Quest1Complete
  (bind _playerinvref (Variables|Default|GetPlayerInvRef))
  (bind _investigator (Variables|Default|GetInvestigator))
  (bind _success (CallFunction|DeleteItemsinAllInventoriesbyTemplateID _investigator (Variables|Default|GetQ1_R_ID) (Variables|Default|GetQ1%20R%20Q)))
  (Utilities|And+Branch _success _success
    (:True
      (Class|ItemInventory|AddItemTemplate _playerinvref (Variables|Default|GetQ1%20Reward) (Class|ItemInventory|GetFirstFreeIndex _playerinvref false) 1 false 1.0 -1.0 :!pinned true) ; Reward
      (Class|ConanCharacter|ClientShowMessage (Variables|Default|GetConChar) (Utilities|Text|MakeLiteralText "Hair of the Dog") (Utilities|Text|MakeLiteralText "The man’s eyes open, at the stench of rotten meat, and he forces himself up.  He lifts the top of the ale cask behind him, shoving the rancid meat within, and then pounding the lid of the barrel back into place with a hand.  He kneels, tapping the bottom of the cask, and a greenish fluid runs from within.  He fills two mugs - and upends the first.  In a moment, he is refreshed - blinking and looking up at the sun and giving a yawn.

He slides the second green concoction across the flimsy stand.  He gives a small smile - and then begins to refill his own mug.  As you eye the mixture hesitantly, he laughs.  “Doesn’t kill you… makes you stronger,” he promises.  
") :!pinned true) ; Complete Text
    )
    (:False
      (bind _asfun_combat_player_controller (Utilities|Casting|CastToFunCombat_PlayerController _investigator))
      (Default|NotificationText _asfun_combat_player_controller "Quest Error" false))))

(fn Quest2Complete
  (bind _playerinvref (Variables|Default|GetPlayerInvRef))
  (bind _investigator (Variables|Default|GetInvestigator))
  (bind _success (CallFunction|DeleteItemsinAllInventoriesbyTemplateID _investigator (Variables|Default|GetQ2%20R%201%20ID) (Variables|Default|GetQ2%20R%201%20Q)))
  (bind _success_2 (CallFunction|DeleteItemsinAllInventoriesbyTemplateID _investigator (Variables|Default|GetQ2%20R%202%20ID) (Variables|Default|GetQ2%20R%202%20Q)))
  (Utilities|And+Branch _success_2 _success
    (:True
      (Class|ItemInventory|AddItemTemplate _playerinvref (Variables|Default|GetQ2%20Reward) (Class|ItemInventory|GetFirstFreeIndex _playerinvref false) 1 false 1.0 -1.0 :!pinned true) ; Reward
      (Class|ConanCharacter|ClientShowMessage (Variables|Default|GetConChar) (Utilities|Text|MakeLiteralText "White Rhino Soup") (Utilities|Text|MakeLiteralText "*Looking at you he licked his lips and dragged the rhino head over to the cauldron, and got to work preparing the almighty soup he promised. The smell is just overwhelming but you can't help as your mouth waters at it. Not being able to see anything else he puts into it you just accept the meal and eat, and soup has never tasted so good.*

((You recieved a White Rhino Soup))") :!pinned true) ; Complete Text
    )
    (:False
      (bind _asfun_combat_player_controller (Utilities|Casting|CastToFunCombat_PlayerController _investigator))
      (Default|NotificationText _asfun_combat_player_controller "Quest Error" false))))