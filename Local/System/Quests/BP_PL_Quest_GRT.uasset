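; Interactable Conan Exiles quest giver (Dakarai) that trades abysmal trophies and currency for trinket rewards.
; On interaction, admins get the parent behavior, while players have their backpack checked for Quest 1's two items, then Quest 2's, else see the quest text.
; Each completion function deletes both requirements from all inventories, then adds the reward and shows story text, or notifies "Quest Error" if either deletion fails.
; BeginPlay switches on the actor's lights.
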(event EventBeginPlay
  (Default|TurnonAll (Variables|Default|GetBP_BAC_TurnLightOnOff))
  (|CallParentFunction))

(event Collision|EventActorBeginOverlap
  (params (OtherActor :type Actor%20Object%20Reference)))

(event EventTick
  (params (DeltaSeconds :type Float%20%28single-precision%29)))

(event EventInteractableActivate
  (params (Component :type Primitive%20Component%20Object%20Reference) (Instigator :type Player%20Controller%20Object%20Reference) (HitIndex :type Integer))
  (bind _output_get (Variables|Default|SetInvestigator Instigator))
  (bind _asconan_player_controller (Utilities|Casting|CastToConanPlayerController _output_get))
  (if (Class|ConanPlayerController|IsAdmin _asconan_player_controller)
    (|CallParentFunction Component Instigator HitIndex)
    (else
      (bind _asconan_character (Utilities|Casting|CastToConanCharacter (Pawn|GetControlledPawn Instigator))
        (:then
          (bind _output_get_2 (Variables|Default|SetConChar _asconan_character))
          (bind _returnvalue (Class|ConanCharacter|GetBackpackInventory _output_get_2))
          (bind _output_get_3 (Variables|Default|SetPlayerInvRef _returnvalue))
          ;[1 1 1] Q1 Requirements
          (Utilities|And+Branch (Class|ItemInventory|HasItembyTemplateID _output_get_3 (Variables|Default|GetQ1_R_ID) (Variables|Default|GetQ1%20R%20Q)) (Class|ItemInventory|HasItembyTemplateID _output_get_3 (Variables|Default|GetQ1%20R%202%20ID) (Variables|Default|GetQ1%20R%202%20Q)) ; Quest1 Item Check
            (:True
              (CallFunction|Quest1Complete))
            (:False
              ;[1 1 1] Q2 Requirements
              (Utilities|And+Branch (Class|ItemInventory|HasItembyTemplateID _output_get_3 (Variables|Default|GetQ2%20R%201%20ID) (Variables|Default|GetQ2%20R%201%20Q)) (Class|ItemInventory|HasItembyTemplateID _output_get_3 (Variables|Default|GetQ2%20R%202%20ID) (Variables|Default|GetQ2%20R%202%20Q)) ; Quest2 Item Check
                (:True
                  (CallFunction|Quest2Complete))
                (:False
                  (Class|ConanCharacter|ClientShowMessage (Variables|Default|GetConChar) (Utilities|Text|MakeLiteralText "Dakarai") (Utilities|Text|MakeLiteralText "A man stares with darkened eyes towards the distant camp of the Dafari.  His eyes don’t stray from it, and a hard rage boils in his eyes.  His gaze doesn’t waver as you approach - his eyes remain locked on the black walls of the ruin behind the Dafari’s camp.  

“She was my everything.”  His voice isn’t broken.  It’s razor sharp steel.  “And that thing took her from me.  Melted in acid til she was soft enough to eat, bewitched by that … damned voice.”  He runs his hand over a small trinket in his hand, a curious piece of jewelry.  A horrifying eye is preserved within amber.  “I want it to hurt.  As much as it hurt her.  I’ll make it worth your while, traveller.”

((500 Abysmal Fang and 100 silver))
((10 Abysmal Eye and 250 golds))") :!pinned true) ; Both Quest Requ is missing
                )))))
        (:CastFailed
          (Development|PrintString "Casto to Conan Character Failed"))))))

(fn ConstructionScript
  (|CallParentFunction))

(fn GetArtisanThrallInventory
  (return (Variables|Default|GetThrallInventory)))

(fn Quest1Complete
  (bind _playerinvref (Variables|Default|GetPlayerInvRef))
  (bind _investigator (Variables|Default|GetInvestigator))
  (bind _success (CallFunction|DeleteItemsinAllInventoriesbyTemplateID _investigator (Variables|Default|GetQ1_R_ID) (Variables|Default|GetQ1%20R%20Q)))
  (bind _success_2 (CallFunction|DeleteItemsinAllInventoriesbyTemplateID _investigator (Variables|Default|GetQ1%20R%202%20ID) (Variables|Default|GetQ1%20R%202%20Q)))
  (Utilities|And+Branch _success_2 _success
    (:True
      (Class|ItemInventory|AddItemTemplate _playerinvref (Variables|Default|GetQ1%20Reward) (Class|ItemInventory|GetFirstFreeIndex _playerinvref false) 1 false 1.0 -1.0 :!pinned true) ; Reward
      (Class|ConanCharacter|ClientShowMessage (Variables|Default|GetConChar) (Utilities|Text|MakeLiteralText "Fang Trinket") (Utilities|Text|MakeLiteralText "The old man looks over the assortment of fangs, a wide smile on his face.  It grows with each bloody fang, and he gives a small nod.  “Vengeance.”  His voice is soft.  “It’s never enough - but sometimes it keeps up going when naught else will.”  He offers a small trophy of your victory, and looks back towards the wall, going silent again.

") :!pinned true) ; Complete Text
    )
    (:False
      (bind _asfun_combat_player_controller (Utilities|Casting|CastToFunCombat_PlayerController _investigator))
      (Default|NotificationText _asfun_combat_player_controller "Quest Error" false))))

(fn Quest2Complete
  (bind _playerinvref (Variables|Default|GetPlayerInvRef))
  (bind _investigator (Variables|Default|GetInvestigator))
  (bind _success (CallFunction|DeleteItemsinAllInventoriesbyTemplateID _investigator (Variables|Default|GetQ2%20R%201%20ID) (Variables|Default|GetQ2%20R%201%20Q)))
  (bind _success_2 (CallFunction|DeleteItemsinAllInventoriesbyTemplateID _investigator (Variables|Default|GetQ2%20R%202%20ID) (Variables|Default|GetQ2%20R%202%20Q)))
  (Utilities|And+Branch _success_2 _success
    (:True
      (Class|ItemInventory|AddItemTemplate _playerinvref (Variables|Default|GetQ2%20Reward) (Class|ItemInventory|GetFirstFreeIndex _playerinvref false) 1 false 1.0 -1.0 :!pinned true) ; Reward
      (Class|ConanCharacter|ClientShowMessage (Variables|Default|GetConChar) (Utilities|Text|MakeLiteralText "Ambar Preserved Eye Jewel") (Utilities|Text|MakeLiteralText "
The old man looks down at the torn eyes, and as if by some hidden knowledge, reaches down for one of the eyes struck free before the beast was dead.  He hefts it with a cold smile, and then plucks a jewel hanging from a chain around his neck.  The infernal eye preserved within glares balefully.  “I heard it scream from here.”  He looks up, and gives a grateful nod.  “Thank you.”
") :!pinned true) ; Complete Text
    )
    (:False
      (bind _asfun_combat_player_controller (Utilities|Casting|CastToFunCombat_PlayerController _investigator))
      (Default|NotificationText _asfun_combat_player_controller "Quest Error" false))))