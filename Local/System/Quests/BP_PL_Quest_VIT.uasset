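; Conan Exiles quest-giver interactable for the witch "Witch Bec", who trades two item turn-in quests for rewards.
; Admins get the parent interaction, while other players have their backpack checked for Quest 1's item pair, then Quest 2's, otherwise seeing the quest dialogue.
; Completion functions delete both items across all inventories, then add the reward with story text and a notification, or report an error.
; BeginPlay switches on its lights.
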(event EventBeginPlay
  (Default|TurnonAll (Variables|Default|GetBP_BAC_TurnLightOnOff)))

(event Collision|EventActorBeginOverlap
  (params (OtherActor :type Actor%20Object%20Reference)))

(event EventTick
  (params (DeltaSeconds :type Float%20%28single-precision%29)))

(event EventInteractableActivate
  (params (Component :type Primitive%20Component%20Object%20Reference) (Instigator :type Player%20Controller%20Object%20Reference) (HitIndex :type Integer))
  (bind _output_get (Variables|Default|SetInvestigator Instigator))
  (bind _asconan_player_controller (Utilities|Casting|CastToConanPlayerController _output_get))
  (if (Class|ConanPlayerController|IsAdmin _asconan_player_controller)
    (|CallParentFunction Component Instigator HitIndex)
    (else
      (bind _asconan_character (Utilities|Casting|CastToConanCharacter (Pawn|GetControlledPawn Instigator)))
      (bind _output_get_2 (Variables|Default|SetConChar _asconan_character))
      (bind _returnvalue (Class|ConanCharacter|GetBackpackInventory _output_get_2))
      (bind _output_get_3 (Variables|Default|SetPlayerInvRef _returnvalue))
      ;[1 1 1] Q1 Requirements
      (Utilities|And+Branch (Class|ItemInventory|HasItembyTemplateID _output_get_3 (Variables|Default|GetQ1_R_ID) (Variables|Default|GetQ1%20R%20Q)) (Class|ItemInventory|HasItembyTemplateID _output_get_3 (Variables|Default|GetQ1%20R%202%20ID) (Variables|Default|GetQ1%20R%202%20Q)) ; Quest1 Item Check
        (:True
          (CallFunction|Quest1Complete))
        (:False
          ;[1 1 1] Q2 Requirements
          (Utilities|And+Branch (Class|ItemInventory|HasItembyTemplateID _output_get_3 (Variables|Default|GetQ2%20R%201%20ID) (Variables|Default|GetQ2%20R%201%20Q)) (Class|ItemInventory|HasItembyTemplateID _output_get_3 (Variables|Default|GetQ2%20R%202%20ID) (Variables|Default|GetQ2%20R%202%20Q)) ; Quest2 Item Check
            (:True
              (CallFunction|Quest2Complete))
            (:False
              (Class|ConanCharacter|ClientShowMessage (Variables|Default|GetConChar) (Utilities|Text|MakeLiteralText "Witch Bec") (Utilities|Text|MakeLiteralText "*You approach a strange looking figure, a woman dressed in bones of animals and bits of cloth. She was humming to herself as she casually explored the insides of a dragon's mouth checking the teeth and structure . Tutting she leaves the dragon's mouth and looks over at you as your approach. Not caring to ask she begins to walk around you looking you over.*
 You'll do, go fetch me some green dragon heads... their eyes should be useful... 
*Deciding it best to not question her you leave to get what she asks. But a hand stops you.*
 The hearts of kings could also be... most helpful.
*She adds staring off into the distance her eyes glassy before letting you go and drifting off around the head of the beast.*
((40 Green Dragon Heads and 100 silver))
((10 Heart of the Kinscourge and 250 gold))
") :!pinned true) ; Both Quest Requ is missing
            )))))))

(fn ConstructionScript
  (|CallParentFunction))

(fn GetArtisanThrallInventory
  (return (Variables|Default|GetThrallInventory)))

(fn Quest1Complete
  (bind _playerinvref (Variables|Default|GetPlayerInvRef))
  (bind _investigator (Variables|Default|GetInvestigator))
  (bind _success (CallFunction|DeleteItemsinAllInventoriesbyTemplateID _investigator (Variables|Default|GetQ1_R_ID) (Variables|Default|GetQ1%20R%20Q)))
  (bind _success_2 (CallFunction|DeleteItemsinAllInventoriesbyTemplateID _investigator (Variables|Default|GetQ1%20R%202%20ID) (Variables|Default|GetQ1%20R%202%20Q)))
  (Utilities|And+Branch _success_2 _success
    (:True
      (Class|ItemInventory|AddItemTemplate _playerinvref (Variables|Default|GetQ1%20Reward) (Class|ItemInventory|GetFirstFreeIndex _playerinvref false) 1 false 1.0 -1.0 :!pinned true) ; Reward
      (Class|ConanCharacter|ClientShowMessage (Variables|Default|GetConChar) (Utilities|Text|MakeLiteralText "Cursed City Spell dust") (Utilities|Text|MakeLiteralText "*As you come back with the heads of dragons, you look upon her you see she is standing there waiting for you. Signalling for you to drop the heads she hands a pouch to you and then dismisses you with a flick of a hand, as her knife sinks into the eye socket of one of the heads.*") :!pinned true) ; Complete Text
      (bind _asfun_combat_player_controller (Utilities|Casting|CastToFunCombat_PlayerController _investigator))
      (Default|NotificationText _asfun_combat_player_controller "Recieved Item:  Cursed City Spell dust" false))
    (:False
      (bind _asfun_combat_player_controller_2 (Utilities|Casting|CastToFunCombat_PlayerController _investigator))
      (Default|NotificationText _asfun_combat_player_controller_2 "Quest Error" false))))

(fn Quest2Complete
  (bind _playerinvref (Variables|Default|GetPlayerInvRef))
  (bind _investigator (Variables|Default|GetInvestigator))
  (bind _success (CallFunction|DeleteItemsinAllInventoriesbyTemplateID _investigator (Variables|Default|GetQ2%20R%201%20ID) (Variables|Default|GetQ2%20R%201%20Q)))
  (bind _success_2 (CallFunction|DeleteItemsinAllInventoriesbyTemplateID _investigator (Variables|Default|GetQ2%20R%202%20ID) (Variables|Default|GetQ2%20R%202%20Q)))
  (Utilities|And+Branch _success_2 _success
    (:True
      (Class|ItemInventory|AddItemTemplate _playerinvref (Variables|Default|GetQ2%20Reward) (Class|ItemInventory|GetFirstFreeIndex _playerinvref false) 1 false 1.0 -1.0 :!pinned true) ; Reward
      (Class|ConanCharacter|ClientShowMessage (Variables|Default|GetConChar) (Utilities|Text|MakeLiteralText "Life Force Offering") (Utilities|Text|MakeLiteralText "Y-you did it?
*She seemed genuinely surprised about this and grinned before clapping her hands together and smiling widely.*
Oh isn't that just wonderful... I could never stand liches... they get in the way. 
*The air turned cold around her as she fixes you with a stare that seems to pierce through your very being.*
I guess that's what people do when they fear death.. they'll just settle for anything.. 
*She took one of the hearts and rolled it around in her hand slowly, taking in the sight of it and the smell, even running her tongue over it once before she tosses them to the side.*
 I... think you've earnt something though.. 
*Leaning in close she slaps her hand onto your chest with a loud bang you feel it burning as a mark flares up on it before vanishing.* 
") :!pinned true) ; Complete Text
      (bind _asfun_combat_player_controller (Utilities|Casting|CastToFunCombat_PlayerController _investigator))
      (Default|NotificationText _asfun_combat_player_controller "Recieved Item:  Life Force Offering" false))
    (:False
      (bind _asfun_combat_player_controller_2 (Utilities|Casting|CastToFunCombat_PlayerController _investigator))
      (Default|NotificationText _asfun_combat_player_controller_2 "Quest Error" false))))