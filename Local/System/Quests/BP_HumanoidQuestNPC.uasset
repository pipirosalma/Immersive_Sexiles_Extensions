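; Humanoid NPC Blueprint for quest givers that players interact with to start dialogue.
; It sets itself to a passive state on spawn and forwards both client and server interactions to its DialogueComponent.
; Activation also logs a "FindstoryNPC" Exiles Journey event on the interacting player's pawn, if that component exists.
; The interaction UI module shows dialogue NPC info, hidden while the client is already in dialogue.
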(event EventBeginPlay
  (|CallParentFunction)
  (Class|ConanCharacter|SetCharacterState "Passive"))

(event EventTick
  (params (DeltaSeconds :type Float%20%28single-precision%29))
  (|CallParentFunction DeltaSeconds))

(event EventClientInteractableActivate
  (params (Component :type Primitive%20Component%20Object%20Reference) (Instigator :type Player%20Controller%20Object%20Reference) (HitIndex :type Integer))
  (Default|ClientInteractableActivate (Variables|Default|GetDialogueComponent) Component Instigator HitIndex))

(event EventInteractableActivate
  (params (Component :type Primitive%20Component%20Object%20Reference) (Instigator :type Player%20Controller%20Object%20Reference) (HitIndex :type Integer))
  (bind _returnvalue (Pawn|GetControlledPawn Instigator))
  (bind _returnvalue_2 (Actor|GetComponentbyClass _returnvalue "/Game/Systems/Progression/BP_AC_ExilesJourney.BP_AC_ExilesJourney_C"))
  (Default|InteractableActivate (Variables|Default|GetDialogueComponent) Component Instigator HitIndex)
  (Utilities|IsValid _returnvalue_2
    (:Is%20Valid
      (Class|ExilesJourneyComponent|AddJourneyEvent _returnvalue_2 "FindstoryNPC" (Transformation|GetActorLocation _returnvalue)))))

(fn ConstructionScript
  (|CallParentFunction))

(fn InteractableGetUIModuleName
  (if (Variables|/Game/Systems/Components/DialogueComponent.DialogueComponent_C|GetClientInDialogue? (Variables|Default|GetDialogueComponent))
    (return "None")
    (else
      (return "DialogueNPCInfo"))))