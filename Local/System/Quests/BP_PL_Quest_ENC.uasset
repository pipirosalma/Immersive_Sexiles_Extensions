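; Interactable merchant quest placeable (Gabai) that trades required items, described as silver or gold payments, for hired-help or mount rewards.
; On interaction, admins get the parent behavior, while other players have their backpack checked for Quest 1, then Quest 2, otherwise seeing the offer dialogue.
; Completion deletes the cost by template ID, adds the reward and shows dialogue, or notifies an error if deletion fails.
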(event EventBeginPlay
  (Default|TurnonAll (Variables|Default|GetBP_BAC_TurnLightOnOff))
  (|CallParentFunction))

(event Collision|EventActorBeginOverlap
  (params (OtherActor :type Actor%20Object%20Reference)))

(event EventTick
  (params (DeltaSeconds :type Float%20%28single-precision%29)))

(event EventInteractableActivate
  (params (Component :type Primitive%20Component%20Object%20Reference) (Instigator :type Player%20Controller%20Object%20Reference) (HitIndex :type Integer))
  (bind _output_get (Variables|Default|SetInvestigator Instigator))
  (bind _asconan_player_controller (Utilities|Casting|CastToConanPlayerController _output_get))
  (if (Class|ConanPlayerController|IsAdmin _asconan_player_controller)
    (|CallParentFunction Component Instigator HitIndex)
    (else
      (bind _asconan_character (Utilities|Casting|CastToConanCharacter (Pawn|GetControlledPawn Instigator))
        (:then
          (bind _output_get_2 (Variables|Default|SetConChar _asconan_character))
          (bind _returnvalue (Class|ConanCharacter|GetBackpackInventory _output_get_2))
          (bind _output_get_3 (Variables|Default|SetPlayerInvRef _returnvalue))
          ;[1 1 1] Q1 Requirements
          (Utilities|And+Branch (Class|ItemInventory|HasItembyTemplateID _output_get_3 (Variables|Default|GetQ1_R_ID) (Variables|Default|GetQ1%20R%20Q)) true ; Quest1 Item Check
            (:True
              (CallFunction|Quest1Complete))
            (:False
              ;[1 1 1] Q2 Requirements
              (Utilities|And+Branch (Class|ItemInventory|HasItembyTemplateID _output_get_3 (Variables|Default|GetQ2%20R%201%20ID) (Variables|Default|GetQ2%20R%201%20Q)) true ; Quest2 Item Check
                (:True
                  (CallFunction|Quest2Complete))
                (:False
                  (Class|ConanCharacter|ClientShowMessage (Variables|Default|GetConChar) (Utilities|Text|MakeLiteralText "Gabai the Humble Merchant") (Utilities|Text|MakeLiteralText "The Shemite smiles as you approach, bowing his head deeply.  “Honorable sir,” he wheedles, his bow deep enough to impress a Sultan.  “This humble merchant offers the finest of wares.  Come, look!  I am certain we have just what you need, alnabil sayidi.”  His eyes linger hungrily on your coin purse, as he pushes forward a pair of contracts for perusal.  

[Gabai the Humblest of Merchants will provide a deaf-mute laborer to ease your burdens and carry your possessions.  Labor no longer like a common mongrel, but relax as well-trained servants fetch and carry for you as for a Shemite Prince!  All laborers are non-refundable.  All laborers are sold as is.  Gabai the Humblest of Merchants is not responsible for theft, mutilation, or death resulting from exposure in the Exiled Lands.  (The contract continues at length, largely insuring Gabai’s immunity to retaliation and offering assurances of the qualities of his wares.  The price is outlandish.)]

[Gabai the Humblest of Merchants will provide a trained pack-hyena to follow you, and carry your possessions without complaint.  Recline in sunshine and happiness, drink fermented beverages while your servants leap to your command with but a whistle.  All hyenas are non-refundable… (This contract is as extensive as the first, and even claims the hyenas can be ridden as a pack-horse.  The price is astronomical.)]

((1000 silver))
((1000 golds))") :!pinned true) ; Both Quest Requ is missing
                )))))
        (:CastFailed
          (Development|PrintString "Casto to Conan Character Failed"))))))

(fn ConstructionScript
  (|CallParentFunction))

(fn GetArtisanThrallInventory
  (return (Variables|Default|GetThrallInventory)))

(fn Quest1Complete
  (bind _playerinvref (Variables|Default|GetPlayerInvRef))
  (bind _investigator (Variables|Default|GetInvestigator))
  (bind _success (CallFunction|DeleteItemsinAllInventoriesbyTemplateID _investigator (Variables|Default|GetQ1_R_ID) (Variables|Default|GetQ1%20R%20Q)))
  (Utilities|And+Branch true _success
    (:True
      (Class|ItemInventory|AddItemTemplate _playerinvref (Variables|Default|GetQ1%20Reward) (Class|ItemInventory|GetFirstFreeIndex _playerinvref false) 1 false 1.0 -1.0 :!pinned true) ; Reward
      (Class|ConanCharacter|ClientShowMessage (Variables|Default|GetConChar) (Utilities|Text|MakeLiteralText "Hired Help") (Utilities|Text|MakeLiteralText "
“Fine!  A thousand silvers!  You rob me, alnabil sayidi, but Gabai has many children to feed.  That is my lowest offer!”  He seems genuinely outraged, even as he gestures for a thrall who looks barely strong enough to stand to approach.  “I hope you are satisfied, sayidi!  You take food from the mouths of my children!”
") :!pinned true) ; Complete Text
    )
    (:False
      (bind _asfun_combat_player_controller (Utilities|Casting|CastToFunCombat_PlayerController _investigator))
      (Default|NotificationText _asfun_combat_player_controller "Quest Error" false))))

(fn Quest2Complete
  (bind _playerinvref (Variables|Default|GetPlayerInvRef))
  (bind _investigator (Variables|Default|GetInvestigator))
  (bind _success (CallFunction|DeleteItemsinAllInventoriesbyTemplateID _investigator (Variables|Default|GetQ2%20R%201%20ID) (Variables|Default|GetQ2%20R%201%20Q)))
  (Utilities|And+Branch true _success
    (:True
      (Class|ItemInventory|AddItemTemplate _playerinvref (Variables|Default|GetQ2%20Reward) (Class|ItemInventory|GetFirstFreeIndex _playerinvref false) 1 false 1.0 -1.0 :!pinned true) ; Reward
      (Class|ConanCharacter|ClientShowMessage (Variables|Default|GetConChar) (Utilities|Text|MakeLiteralText "Mounted Travel") (Utilities|Text|MakeLiteralText "
“A thousand gold?  I might as well begin breaking stone with my own two hands, if that is all you will offer this humble merchant.  Look at his magnificent beast!  It will battle your foes!  Carry you to war!  Cart your burdens without complaint!  And you would offer but a thousand pieces?  The sultan would have paid a boatload of silks for such a steed!”  He shakes his head in exasperation.  “Fine!  Fine, but I will not 
") :!pinned true) ; Complete Text
    )
    (:False
      (bind _asfun_combat_player_controller (Utilities|Casting|CastToFunCombat_PlayerController _investigator))
      (Default|NotificationText _asfun_combat_player_controller "Quest Error" false))))