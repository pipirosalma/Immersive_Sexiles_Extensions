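; Knockout debuff state that plays a knockout animation on the instigating player's controlled character when the buff starts.
; On start it resolves the pawn through the instigator's combat player controller and passes an unconscious duration to its additional-animations component.
; That duration shrinks as the owning character's Metabolism stat rises, and the player's combat state is then updated.
; Clearing on the client only defers to the parent buff.
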(event EventStartBuff
  (params (BuffPotency :type Integer) (DamageCauser :type Actor%20Object%20Reference) (OwningCharacter :type Conan%20Character%20Object%20Reference) (Instigator :type Controller%20Object%20Reference))
  (|CallParentFunction BuffPotency DamageCauser OwningCharacter Instigator)
  (bind _asfun_combat_player_controller (Utilities|Casting|CastToFunCombat_PlayerController Instigator))
  (bind _asbase_player_char (Utilities|Casting|CastToBasePlayerChar (Pawn|GetControlledPawn _asfun_combat_player_controller)))
  (Default|PlayKnockoutAnimation (Actor|GetComponentbyClass _asbase_player_char "/Game/Mods/Immersive_Sexiles_Extensions/ac_AditionalAnimations.ac_AditionalAnimations_C") OwningCharacter _asbase_player_char (Math|Conversions|ToFloat(Integer) (- 30 (/ (Class|ConanCharacter|GetIntStat OwningCharacter "AttributeMetabolism" "Full") 3))))
  (Default|HandleCombatState _asbase_player_char))

(event EventClientClearBuff
  (params (OwningCharacter :type Conan%20Character%20Object%20Reference))
  (|CallParentFunction OwningCharacter))