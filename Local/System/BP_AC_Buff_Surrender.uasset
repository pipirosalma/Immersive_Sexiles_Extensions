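; Buff component that puts a player character into a surrendered state.
; On start it runs the parent logic, ends active healing and sparring-hit buffs through the character's buff system, and unequips the hands.
; It then enables avoidance invulnerability and triggers Surrender on the character's additional-animations component.
; Clearing the buff only disables that invulnerability.
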(event EventStartBuff
  (params (BuffPotency :type Integer) (DamageCauser :type Actor%20Object%20Reference) (OwningCharacter :type Conan%20Character%20Object%20Reference) (Instigator :type Controller%20Object%20Reference))
  (|CallParentFunction BuffPotency DamageCauser OwningCharacter Instigator)
  (bind _asbase_player_char (Utilities|Casting|CastToBasePlayerChar (Variables|Default|GetOwningCharacter)))
  (Default|EndBuff (Variables|/Game/Characters/BaseBPCombat.BaseBPCombat_C|Get00_BP_AC_BuffSystem _asbase_player_char) "/Game/Systems/Buffs/Heal_OverTime/BP_AC_Buff_Healing_HeartyMeal.BP_AC_Buff_Healing_HeartyMeal_C")
  (Default|EndBuff (Variables|/Game/Characters/BaseBPCombat.BaseBPCombat_C|Get00_BP_AC_BuffSystem _asbase_player_char) "/Game/Systems/Buffs/Heal_OverTime/BP_AC_Buff_HealingPotion_Small.BP_AC_Buff_HealingPotion_Small_C")
  (Default|EndBuff (Variables|/Game/Characters/BaseBPCombat.BaseBPCombat_C|Get00_BP_AC_BuffSystem _asbase_player_char) "/Game/Systems/Buffs/Heal_OverTime/BP_AC_Buff_HealingPotion.BP_AC_Buff_HealingPotion_C")
  (Default|EndBuff (Variables|/Game/Characters/BaseBPCombat.BaseBPCombat_C|Get00_BP_AC_BuffSystem _asbase_player_char) "/Game/Mods/Immersive_Sexiles_Extensions/Assets/Weapons/00_BP_AC_Sparring_Hit.00_BP_AC_Sparring_Hit_C")
  (Default|CallUnequipHands _asbase_player_char)
  (Default|EnableAvoidanceInvulnerability _asbase_player_char)
  (Default|Surrender (Utilities|Array|Get(acopy) (Actor|GetComponentsByClass _asbase_player_char "/Game/Mods/Immersive_Sexiles_Extensions/ac_AditionalAnimations.ac_AditionalAnimations_C")) _asbase_player_char))

(event EventClearBuff
  (bind _asbase_player_char (Utilities|Casting|CastToBasePlayerChar (Variables|Default|GetOwningCharacter)))
  (Default|DisableAvoidanceInvulnerability _asbase_player_char))