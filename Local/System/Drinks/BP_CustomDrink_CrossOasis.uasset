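; Custom Cross Oasis drink item that is always usable and can knock the drinker unconscious depending on drunkenness.
; On use it overwrites its buff application chances: maximum when heavily drunk, otherwise a clamped value that falls as food level and Metabolism rise.
; Heavy drunkenness gives a coin-flip blackout, while lower stages roll drunk stage against Metabolism plus a random value.
; The parent item logic then runs with the adjusted chances.
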(event EventOnUseItem
  (params (invokingCharacter :type Conan%20Character%20Object%20Reference))
  (bind _returnvalue (Actor|GetComponentsByClass invokingCharacter "/Game/Mods/Immersive_Sexiles_Extensions/ac_AditionalAnimations.ac_AditionalAnimations_C"))
  (bind _buff_application_chance (Variables|Default|GetBuff%20Application%20Chance))
  (bind _buff_application_chance_2 (Variables|Default|GetBuff%20Application%20Chance))
  (bind _item (Utilities|Array|Get(acopy) _returnvalue))
  (bind _drunkstage (Variables|/Game/Mods/Immersive_Sexiles_Extensions/ac_AditionalAnimations.ac_AditionalAnimations_C|GetDrunkStage _item))
  (bind _returnvalue_2 (Class|ConanCharacter|GetHungerSystem invokingCharacter))
  (bind _value (Class|BPIHungerSystem|GetFoodCurrent(Message) _returnvalue_2))
  (if (>= _drunkstage 5)
    (for _array_element _buff_application_chance
      (Utilities|Array|SetArrayElem _buff_application_chance 0 (Math|Float|MakeLiteralFloat 1.0)))
    (if (== (Math|Random|RandomIntegerinRange 0 1) 0)
      (bind _asbase_player_char (Utilities|Casting|CastToBasePlayerChar invokingCharacter :!label _label)
        (:then
          (Default|SetPlayerUnconscious (Utilities|Array|Get(acopy) (Actor|GetComponentsByClass _asbase_player_char "/Game/Mods/Immersive_Sexiles_Extensions/ac_AditionalAnimations.ac_AditionalAnimations_C")) _asbase_player_char))
        (:CastFailed
          _)))
    (else
      (for (_ _array_index) _buff_application_chance_2
        (Utilities|Array|SetArrayElem _buff_application_chance_2 _array_index (Math|Float|Clamp(Float) (+ (- 1.0 (/ _value 1e+02)) (- 1.0 (/ (Math|Conversions|ToFloat(Integer) (Class|ConanCharacter|GetIntStat invokingCharacter "AttributeMetabolism" "Full")) 2.5e+02))) 0.2)))
      (if (> (+ 5 _drunkstage) (+ (/ (Class|ConanCharacter|GetIntStat invokingCharacter "AttributeMetabolism" "Full") 10) (Math|Random|RandomIntegerinRange 0 20)))
        (goto _label)
        (else
          _))))
  (|CallParentFunction invokingCharacter))

(fn CanUseItem
  (params (invokingCharacter :type Conan%20Character%20Object%20Reference))
  (return true))