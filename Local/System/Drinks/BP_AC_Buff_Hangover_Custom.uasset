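; Hangover buff, apparently an actor component, that penalizes the owning character's stamina and hydration.
; Buff start lowers max stamina through a merged stat modifier, and clearing applies the opposite modifier to restore it.
; Each buff tick, for player characters only, it reads the current drink level from the hunger system interface and reduces it by a small percentage of itself.
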(event EventGameplayEffecttoApplyonBuffStart
  (Class|ConanCharacter|AddIntStatModifier (Variables|Default|GetOwningCharacter) "StaminaMax" "Buff" "Add" -20 "Merge"))

(event EventGameplayEffecttoApplyonBuffCleared
  (Class|ConanCharacter|AddIntStatModifier (Variables|Default|GetOwningCharacter) "StaminaMax" "Buff" "Add" 20 "Merge"))

(event EventGameplayEffecttoApplyonBuffTick
  (bind _asbase_player_char (Utilities|Casting|CastToBasePlayerChar (Variables|Default|GetOwningCharacter)))
  (bind _returnvalue (Class|ConanCharacter|GetHungerSystem (Variables|Default|GetOwningCharacter)))
  (Utilities|IsValid _returnvalue
    (:Is%20Valid
      (bind _asbpi_hunger_system (Utilities|Casting|CastToBPI_HungerSystem _returnvalue))
      (bind _value (Default|GetDrinkCurrent _asbpi_hunger_system))
      (Default|SetDrinkCurrent (Variables|/Game/Characters/BasePlayerChar.BasePlayerChar_C|GetBP_HungerSystem _asbase_player_char) _value (- _value (* _value 0.01))))))