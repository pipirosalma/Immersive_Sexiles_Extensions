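; Base Blueprint for custom drink items that can always be used and can knock out a drunk character.
; On use, it overwrites each buff application chance with a clamped value that rises as food level and Metabolism fall.
; It then rolls Metabolism plus a d20-style random value against DrunkStage, applying unconsciousness and its debuff to player characters on failure.
; The parent use logic runs last, and a DrunkStage threshold branch is left empty.
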(event EventOnUseItem
  (params (invokingCharacter :type Conan%20Character%20Object%20Reference))
  (bind _returnvalue (Actor|GetComponentsByClass invokingCharacter "/Game/Mods/Immersive_Sexiles_Extensions/ac_AditionalAnimations.ac_AditionalAnimations_C"))
  (bind _buff_application_chance (Variables|Default|GetBuff%20Application%20Chance))
  (bind _item (Utilities|Array|Get(acopy) _returnvalue))
  (bind _drunkstage (Variables|/Game/Mods/Immersive_Sexiles_Extensions/ac_AditionalAnimations.ac_AditionalAnimations_C|GetDrunkStage _item))
  (bind _returnvalue_2 (Class|ConanCharacter|GetHungerSystem invokingCharacter))
  (bind _value (Class|BPIHungerSystem|GetFoodCurrent(Message) _returnvalue_2))
  (if (>= _drunkstage 5)
    _
    (else
      _))
  (for (_ _array_index) _buff_application_chance
    (Utilities|Array|SetArrayElem _buff_application_chance _array_index (Math|Float|Clamp(Float) (+ (- 1.0 (/ _value 1e+02)) (- 1.0 (/ (Math|Conversions|ToFloat(Integer) (Class|ConanCharacter|GetIntStat invokingCharacter "AttributeMetabolism" "Full")) 6e+01))) 0.01)))
  (if (> (+ 0 _drunkstage) (+ (/ (Class|ConanCharacter|GetIntStat invokingCharacter "AttributeMetabolism" "Full") 5) (Math|Random|RandomIntegerinRange 1 20)))
    (bind _asbase_player_char (Utilities|Casting|CastToBasePlayerChar invokingCharacter)
      (:then
        (Default|SetPlayerUnconscious (Utilities|Array|Get(acopy) (Actor|GetComponentsByClass _asbase_player_char "/Game/Mods/Immersive_Sexiles_Extensions/ac_AditionalAnimations.ac_AditionalAnimations_C")) _asbase_player_char)
        (Default|AddBuff (Variables|/Game/Characters/BaseBPCombat.BaseBPCombat_C|Get00_BP_AC_BuffSystem _asbase_player_char) "/Game/Mods/Immersive_Sexiles_Extensions/System/BP_AC_Debuff_Unconscious_State.BP_AC_Debuff_Unconscious_State_C"))
      (:CastFailed
        _)))
  (|CallParentFunction invokingCharacter))

(fn CanUseItem
  (params (invokingCharacter :type Conan%20Character%20Object%20Reference))
  (return true))