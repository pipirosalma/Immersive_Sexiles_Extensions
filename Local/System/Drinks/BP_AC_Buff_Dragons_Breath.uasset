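; Actor component buff for the Dragon's Breath drink that switches custom drink effects on the player character who receives it.
; On start it runs the parent buff logic, then triggers the drink's effect through the character's Ac_AditionalAnimations component.
; When the buff clears it calls the same CustomDrinkEffects function with a different index.
; Both paths act only when the owner is a BasePlayerChar.
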(event EventGameplayEffecttoApplyonBuffCleared
  (bind _asbase_player_char (Utilities|Casting|CastToBasePlayerChar (Variables|Default|GetOwningCharacter)))
  (Default|CustomDrinkEffects (Utilities|Array|Get(acopy) (Actor|GetComponentsByClass _asbase_player_char "/Game/Mods/Immersive_Sexiles_Extensions/ac_AditionalAnimations.ac_AditionalAnimations_C")) 4))

(event EventStartBuff
  (params (BuffPotency :type Integer) (DamageCauser :type Actor%20Object%20Reference) (OwningCharacter :type Conan%20Character%20Object%20Reference) (Instigator :type Controller%20Object%20Reference))
  (|CallParentFunction BuffPotency DamageCauser OwningCharacter Instigator)
  (bind _asbase_player_char (Utilities|Casting|CastToBasePlayerChar (Variables|Default|GetOwningCharacter)))
  (Default|CustomDrinkEffects (Utilities|Array|Get(acopy) (Actor|GetComponentsByClass _asbase_player_char "/Game/Mods/Immersive_Sexiles_Extensions/ac_AditionalAnimations.ac_AditionalAnimations_C"))))