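; Collar armor item that toggles collared animation state on the player character wearing it.
; On equip it sets IsCollared on the owner's first Ac_AditionalAnimations component, if one exists.
; On unequip it clears both IsCollared and IsCaptured on that component, and both events then call the parent equip logic.
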(event EventOnEquip
  (params (owner :type Character%20Object%20Reference))
  (bind _asbase_player_char (Utilities|Casting|CastToBasePlayerChar owner)
    (:then
      (if (> (Utilities|Array|Length (Actor|GetComponentsByClass _asbase_player_char "/Game/Mods/Immersive_Sexiles_Extensions/ac_AditionalAnimations.ac_AditionalAnimations_C")) 0)
        (Variables|/Game/Mods/Immersive_Sexiles_Extensions/ac_AditionalAnimations.ac_AditionalAnimations_C|SetIsCollared (Utilities|Array|Get(acopy) (Actor|GetComponentsByClass _asbase_player_char "/Game/Mods/Immersive_Sexiles_Extensions/ac_AditionalAnimations.ac_AditionalAnimations_C")) true)))
    (:CastFailed
      _))
  (|CallParentFunction owner))

(event EventOnUnEquip
  (params (owner :type Character%20Object%20Reference))
  (bind _asbase_player_char (Utilities|Casting|CastToBasePlayerChar owner)
    (:then
      (if (> (Utilities|Array|Length (Actor|GetComponentsByClass _asbase_player_char "/Game/Mods/Immersive_Sexiles_Extensions/ac_AditionalAnimations.ac_AditionalAnimations_C")) 0)
        (Variables|/Game/Mods/Immersive_Sexiles_Extensions/ac_AditionalAnimations.ac_AditionalAnimations_C|SetIsCollared (Utilities|Array|Get(acopy) (Actor|GetComponentsByClass _asbase_player_char "/Game/Mods/Immersive_Sexiles_Extensions/ac_AditionalAnimations.ac_AditionalAnimations_C")) false)
        (Variables|/Game/Mods/Immersive_Sexiles_Extensions/ac_AditionalAnimations.ac_AditionalAnimations_C|SetIsCaptured (Utilities|Array|Get(acopy) (Actor|GetComponentsByClass _asbase_player_char "/Game/Mods/Immersive_Sexiles_Extensions/ac_AditionalAnimations.ac_AditionalAnimations_C")) false)))
    (:CastFailed
      _))
  (|CallParentFunction owner))