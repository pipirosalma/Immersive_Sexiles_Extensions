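; Handcuff equippable that puts its wearer into a bound pose, cycling AnimSequence through behind-back, kneeling and ground poses on successive equips.
; Equipping plays the pose through the player's Ac_AditionalAnimations component; the two non-zero poses also block move input and add the handcuffed buff.
; Unequipping stops the bound montages, removes the buff and restores movement.
; AnimSequence has an empty OnRep, and the direct-montage AnimCall macro is unused here.
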(event EventOnEquip
  (params (owner :type Character%20Object%20Reference))
  (bind _returnvalue (Pawn|GetController owner))
  (|CallParentFunction owner)
  (if (== (Variables|Default|GetAnimSequence) 2)
    (Variables|Default|SetAnimSequence 0)
    (else
      (bind _result (Math|Integer|IncrementInt (Variables|Default|GetAnimSequence))
        (:%20%20
          (Variables|Default|SetAnimSequence _result)))))
  (bind _item (Utilities|GetAditionalAnimComp)
    (:then
      (Utilities|NewMacro0 _item _item _item owner owner owner
        (:then
          _)
        (:then2
          _)
        (:then3
          _))
      (bind _asbase_bpcombat (Utilities|Casting|CastToBaseBPCombat owner))
      (if (!= (Variables|Default|GetAnimSequence) 0)
        (Input|SetIgnoreMoveInput _returnvalue true)
        (Default|AddBuff (Variables|/Game/Characters/BaseBPCombat.BaseBPCombat_C|Get00_BP_AC_BuffSystem _asbase_bpcombat) "/Game/Mods/Immersive_Sexiles_Extensions/Assets/Armors/Chains/BP_AC_Buff_handcuffed.BP_AC_Buff_handcuffed_C" owner 0 _returnvalue)))))

(event EventOnUnEquip
  (params (owner :type Character%20Object%20Reference))
  (|CallParentFunction owner)
  (Animation|StopAnimMontage owner "/Game/Mods/Immersive_Sexiles_Extensions/Assets/Animation/AM_emote_bound_sleeping_ground.AM_emote_bound_sleeping_ground")
  (Animation|StopAnimMontage owner "/Game/Mods/Immersive_Sexiles_Extensions/Assets/Animation/AM_emote_bound_kneeling.AM_emote_bound_kneeling")
  (Animation|StopAnimMontage owner "/Game/Mods/Immersive_Sexiles_Extensions/Assets/Animation/AM_Behind_Back_Bound.AM_Behind_Back_Bound")
  (bind _asbase_bpcombat (Utilities|Casting|CastToBaseBPCombat owner))
  (Default|RemoveBuff (Variables|/Game/Characters/BaseBPCombat.BaseBPCombat_C|Get00_BP_AC_BuffSystem _asbase_bpcombat) "/Game/Mods/Immersive_Sexiles_Extensions/Assets/Armors/Chains/BP_AC_Buff_handcuffed.BP_AC_Buff_handcuffed_C")
  (Input|SetIgnoreMoveInput (Pawn|GetController owner) false))

(fn OnRepAnimSequence)