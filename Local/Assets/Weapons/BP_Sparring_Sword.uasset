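; BP_Sparring_Sword is a weapon Blueprint that puts its combat-character owner into a sparring state while equipped.
; On equip, it calls the parent logic, adds the 00_BP_AC_Sparring buff and stores the owner's max health as SparringPreviousHP on its Ac_RPC_Component.
; On unequip, it calls the parent logic, removes the buff and resets that stored value to -1.
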(event EventOnEquip
  (params (owner :type Character%20Object%20Reference))
  (|CallParentFunction owner)
  (bind _asbase_bpcombat (Utilities|Casting|CastToBaseBPCombat owner))
  (Default|AddBuff (Variables|/Game/Characters/BaseBPCombat.BaseBPCombat_C|Get00_BP_AC_BuffSystem _asbase_bpcombat) "/Game/Mods/Immersive_Sexiles_Extensions/Assets/Weapons/00_BP_AC_Sparring.00_BP_AC_Sparring_C" owner 0 (Pawn|GetController owner))
  (Variables|/Game/Mods/Immersive_Sexiles_Extensions/ac_RPC_Component.ac_RPC_Component_C|SetSparringPreviousHP (Utilities|Array|Get(acopy) (Actor|GetComponentsByClass _asbase_bpcombat "/Game/Mods/Immersive_Sexiles_Extensions/ac_RPC_Component.ac_RPC_Component_C")) (Default|GetHealthMax _asbase_bpcombat)))

(event EventOnUnEquip
  (params (owner :type Character%20Object%20Reference))
  (|CallParentFunction owner)
  (bind _asbase_bpcombat (Utilities|Casting|CastToBaseBPCombat owner))
  (Default|RemoveBuff (Variables|/Game/Characters/BaseBPCombat.BaseBPCombat_C|Get00_BP_AC_BuffSystem _asbase_bpcombat) "/Game/Mods/Immersive_Sexiles_Extensions/Assets/Weapons/00_BP_AC_Sparring.00_BP_AC_Sparring_C")
  (Variables|/Game/Mods/Immersive_Sexiles_Extensions/ac_RPC_Component.ac_RPC_Component_C|SetSparringPreviousHP (Utilities|Array|Get(acopy) (Actor|GetComponentsByClass _asbase_bpcombat "/Game/Mods/Immersive_Sexiles_Extensions/ac_RPC_Component.ac_RPC_Component_C")) -1))