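; One-handed rope weapon Blueprint that visually tethers a victim (thrall) to the actor holding it.
; PlayerRopeSetUp snaps the Cable to the victim's neck bone, then ties that bone to SphereTetherPoint with left and right physics constraints.
; The tether point starts at the victim's location in absolute world space.
; Except on dedicated servers, Tick eases it toward a point below the owner, scaled by delta time.
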(event Custom|PlayerRopeSetUp
  (params (PlayerActor :type Actor%20Object%20Reference) (VictimActor :type Actor%20Object%20Reference))
  (bind _spheretetherpoint (Variables|Default|GetSphereTetherPoint))
  (bind _physicsconstraintleft (Variables|Default|GetPhysicsConstraintLeft))
  (bind _physicsconstraintright (Variables|Default|GetPhysicsConstraintRight))
  (bind _spheretetherpoint_2 (Variables|Default|GetSphereTetherPoint))
  (Variables|Default|SetNewVar_0 VictimActor)
  (bind _returnvalue (Transformation|AttachComponentToComponent (Variables|Default|GetCable) (Utilities|Array|Get(acopy) (Actor|GetComponentsByClass VictimActor "/Script/Engine.SkeletalMeshComponent")) "b_neck_2" "SnapToTarget" "SnapToTarget" "SnapToTarget" true))
  (if _returnvalue
    (if (Networking|IsDedicatedServer)
      _
      (else
        _))
    (bind _output_get (Variables|Default|SetThrall%20Mesh (Utilities|Array|Get(acopy) (Actor|GetComponentsByClass VictimActor "/Script/Engine.SkeletalMeshComponent"))))
    (Class|PhysicsConstraintComponent|SetConstrainedComponents _physicsconstraintleft _spheretetherpoint "None" _output_get "b_neck_2")
    (Class|PhysicsConstraintComponent|SetConstrainedComponents _physicsconstraintright _spheretetherpoint "None" _output_get "b_neck_2")
    (Class|PhysicsConstraintComponent|SetConstraintReferencePosition _physicsconstraintleft "Frame2" (Math|Vector|MakeVector -5.0 0.0 4e+01))
    (Class|PhysicsConstraintComponent|SetConstraintReferencePosition _physicsconstraintright "Frame2" (Math|Vector|MakeVector 5.0 0.0 -4e+01))
    (Class|PhysicsConstraintComponent|SetDisableCollision _physicsconstraintleft true)
    (Class|PhysicsConstraintComponent|SetDisableCollision _physicsconstraintright true)
    (Transformation|SetAbsolute _spheretetherpoint_2 true false false)
    (Transformation|SetWorldLocation _spheretetherpoint_2 (Transformation|GetActorLocation VictimActor) false true)))

(event EventTick
  (params (DeltaSeconds :type Float%20%28single-precision%29))
  (bind _spheretetherpoint (Variables|Default|GetSphereTetherPoint))
  (if (not (Networking|IsDedicatedServer))
    (Transformation|AddRelativeLocation _spheretetherpoint (* (- (- (Transformation|GetActorLocation (Components|GetOwner)) "0, 0,80.000000") (Transformation|GetWorldLocation _spheretetherpoint)) DeltaSeconds) false false)))

(event EventBeginPlay
  (|CallParentFunction))

(fn ConstructionScript
  (|CallParentFunction))