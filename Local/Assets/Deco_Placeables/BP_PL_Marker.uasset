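; Placeable decoration marker that changes its static mesh material when interacted with.
; Each client interact activation steps a three-state material index with wraparound, then calls the parent handler.
; Two states apply the tactician table-top material and the third applies a blue-tinted Oberyn flag material.
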(event EventClientInteractableActivate
  (params (Component :type Primitive%20Component%20Object%20Reference) (Instigator :type Player%20Controller%20Object%20Reference) (HitIndex :type Integer))
  (bind _staticmesh (Variables|Default|GetStaticMesh))
  (if (== (Variables|Default|GetMaterialIndex) 3)
    (Variables|Default|SetMaterialIndex 0))
  (switch int (Variables|Default|GetMaterialIndex)
    (:Default
      (Rendering|Material|SetMaterial _staticmesh 0 "/Game/Mods/Immersive_Sexiles_Extensions/Assets/Deco_Placeables/Cartography/MI_Tactician_Table_Top.MI_Tactician_Table_Top" :!label _label))
    (:0
      (Rendering|Material|SetMaterial _staticmesh 0 "/Game/Mods/Immersive_Sexiles_Extensions/Assets/Deco_Placeables/Cartography/MI_Tactician_Table_Top.MI_Tactician_Table_Top"))
    (:1
      (goto _label))
    (:2
      (Rendering|Material|SetMaterial _staticmesh 0 "/Game/Mods/Immersive_Sexiles_Extensions/Assets/Clan_Banners/Banner_Textures/MI_flags_Oberyn_tint_blue.MI_flags_Oberyn_tint_blue")))
  (Math|Integer|IncrementInt (Variables|Default|GetMaterialIndex)
    (:%20%20
      (|CallParentFunction 0 0 0))))

(event EventBeginPlay)

(event Collision|EventActorBeginOverlap
  (params (OtherActor :type Actor%20Object%20Reference)))

(event EventTick
  (params (DeltaSeconds :type Float%20%28single-precision%29)))

(fn ConstructionScript
  (|CallParentFunction))