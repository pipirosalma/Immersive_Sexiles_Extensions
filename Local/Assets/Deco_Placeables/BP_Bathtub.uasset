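; BP_Bathtub is an interactable bathtub decoration placeable whose effects switch on and off when used.
; Its ClientInteractableActivate event toggles the active state of the steam component, several particle systems and several point lights.
; An unconnected chain, which never runs, would move the player's character to a helper location through an additional-animations component.
; Tick and BeginPlay are unused, and construction only calls the parent script.
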(event EventBeginPlay)

(event Collision|EventActorBeginOverlap
  (params (OtherActor :type Actor%20Object%20Reference)))

(event EventTick
  (params (DeltaSeconds :type Float%20%28single-precision%29)))

(event EventClientInteractableActivate
  (params (Component :type Primitive%20Component%20Object%20Reference) (Instigator :type Player%20Controller%20Object%20Reference) (HitIndex :type Integer))
  (Components|Activation|ToggleActive (Variables|Default|Getsteam))
  (Components|Activation|ToggleActive (Variables|Default|GetParticleSystem))
  (Components|Activation|ToggleActive (Variables|Default|GetPointLight))
  (Components|Activation|ToggleActive (Variables|Default|GetPointLight1))
  (Components|Activation|ToggleActive (Variables|Default|GetParticleSystem1))
  (Components|Activation|ToggleActive (Variables|Default|GetPointLight2))
  (Components|Activation|ToggleActive (Variables|Default|GetParticleSystem2))
  (Components|Activation|ToggleActive (Variables|Default|GetPointLight3))
  (Components|Activation|ToggleActive (Variables|Default|GetParticleSystem3)))

(fn ConstructionScript
  (|CallParentFunction))