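; Placeable dishware of food that players interact with to eat, with a limited number of charges shown as chicken leg meshes.
; On activation, if charges remain and the pawn has a BP_HungerSystem, it spawns a fixed game item and feeds it through ServerGiveFood.
; It then decrements Charges, destroys the matching mesh and plays the eat montage on the player character.
; An unconnected catch-up loop for syncing mesh visibility to Charges never runs.
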(event Custom|SetChickenLegVisibility
  (params (charges :type Integer))
  (switch int charges
    (:0
      (Components|DestroyComponent (Variables|Default|GetStaticMesh1)))
    (:1
      (Components|DestroyComponent (Variables|Default|GetStaticMesh2)))
    (:2
      (Components|DestroyComponent (Variables|Default|GetStaticMesh3)))
    (:3
      (Components|DestroyComponent (Variables|Default|GetStaticMesh4)))
    (:4
      (Components|DestroyComponent (Variables|Default|GetStaticMesh5)))
    (:5
      (Components|DestroyComponent (Variables|Default|GetStaticMesh6)))
    (:6
      (Components|DestroyComponent (Variables|Default|GetStaticMesh7)))
    (:7
      (Components|DestroyComponent (Variables|Default|GetStaticMesh8)))
    (:8
      (Components|DestroyComponent (Variables|Default|GetStaticMesh9)))
    (:9
      (Components|DestroyComponent (Variables|Default|GetStaticMesh10)))
    (:10
      (Components|DestroyComponent (Variables|Default|GetStaticMesh11)))
    (:11
      (Components|DestroyComponent (Variables|Default|GetStaticMesh12)))
    (:12
      (Components|DestroyComponent (Variables|Default|GetStaticMesh13)))
    (:13
      (Components|DestroyComponent (Variables|Default|GetStaticMesh14)))
    (:14
      (Components|DestroyComponent (Variables|Default|GetStaticMesh15)))))

(event Custom|AnimToPlay
  (params (BasePlayerChar :type Base%20Player%20Char%20Object%20Reference))
  (Animation|PlayAnimMontage BasePlayerChar "/Game/Mods/Immersive_Sexiles_Extensions/Assets/Animation/AM_Eat.AM_Eat" 1.0 "None"))

(event Custom|ReduceCharges
  (Variables|Default|SetCharges (- (Variables|Default|GetCharges) 1)))

(event EventInteractableActivate
  (params (Component :type Primitive%20Component%20Object%20Reference) (Instigator :type Player%20Controller%20Object%20Reference) (HitIndex :type Integer))
  (bind _returnvalue (Pawn|GetControlledPawn Instigator))
  (bind _returnvalue_2 (Actor|GetComponentsByClass _returnvalue "/Game/Systems/Hunger/BP_HungerSystem.BP_HungerSystem_C"))
  (if (> (Variables|Default|GetCharges) 0)
    (if (> (Utilities|Array|Length _returnvalue_2) 0)
      (bind _returnvalue_3 (Class|GameItemSpawner|SpawnGameItem 18247))
      (Default|ServerGiveFood (Utilities|Array|Get(acopy) _returnvalue_2) _returnvalue_3 0.0)
      (CallFunction|ReduceCharges)
      (CallFunction|SetChickenLegVisibility (Variables|Default|GetCharges))
      (bind _asbase_player_char (Utilities|Casting|CastToBasePlayerChar _returnvalue))
      (CallFunction|AnimtoPlay _asbase_player_char))))

(event EventBeginPlay)

(event Collision|EventActorBeginOverlap
  (params (OtherActor :type Actor%20Object%20Reference)))

(fn ConstructionScript
  (|CallParentFunction))