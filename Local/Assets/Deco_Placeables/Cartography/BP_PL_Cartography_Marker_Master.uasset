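; Master Blueprint for a placeable cartography marker whose tint color the player cycles by interacting with it.
; BeginPlay applies the stored color to the mesh's tint-mask material parameter.
; Each interaction advances through yellow, red, white and black, then hands the marker, parameter name and color to the player's Ac_AditionalAnimations component via SetMaterials.
; SetColorVector only updates the stored color, without touching the mesh.
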(event Custom|SetColorVector
  (params (NewParam :type Vector))
  (Variables|Default|SetRGBParamValue NewParam))

(event EventInteractableActivate
  (params (Component :type Primitive%20Component%20Object%20Reference) (Instigator :type Player%20Controller%20Object%20Reference) (HitIndex :type Integer))
  (bind _asfun_combat_player_controller (Utilities|Casting|CastToFunCombat_PlayerController Instigator))
  (bind _asbase_player_char (Utilities|Casting|CastToBasePlayerChar (Pawn|GetControlledPawn _asfun_combat_player_controller)))
  (if (> (Utilities|Array|Length (Actor|GetComponentsByClass _asbase_player_char "/Game/Mods/Immersive_Sexiles_Extensions/ac_AditionalAnimations.ac_AditionalAnimations_C")) 0)
    (CallFunction|MaterialSelection)
    (Default|SetMaterials (Utilities|Array|Get(acopy) (Actor|GetComponentsByClass _asbase_player_char "/Game/Mods/Immersive_Sexiles_Extensions/ac_AditionalAnimations.ac_AditionalAnimations_C")) self (Variables|Default|GetTintmaskParamName) (Variables|Default|GetRGBParamValue))))

(event EventBeginPlay
  (Rendering|Material|SetVectorParameterValueonMaterials (Variables|Default|GetStaticMesh) (Variables|Default|GetTintmaskParamName) (Variables|Default|GetRGBParamValue)))

(fn ConstructionScript
  (|CallParentFunction))

(fn MaterialSelection
  (switch int (Variables|Default|GetMaterialSelectionIndex)
    (:Default
      (Variables|Default|SetMaterialSelectionIndex 0)
      (Variables|Default|SetRGBParamValue "1.000000,0.810000, 0" :!label _label))
    (:0
      (goto _label))
    (:1
      (Variables|Default|SetRGBParamValue "1.000000,0.046000,0.000000"))
    (:2
      (Variables|Default|SetRGBParamValue "1.000000,1.000000,1.000000"))
    (:3
      (Variables|Default|SetRGBParamValue "0.000000,0.000000,0.000000")))
  (Math|Integer|IncrementInt (Variables|Default|GetMaterialSelectionIndex)))