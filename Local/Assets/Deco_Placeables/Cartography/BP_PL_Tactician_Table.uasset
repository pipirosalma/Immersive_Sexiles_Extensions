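; Tactician's table placeable that keeps adding three fixed item templates to its own inventory.
; Tick calls SpawnResultItem for each template ID on every update.
; That function adds the item when a slot is free; otherwise it advances a search index through matching stacks, adding only if one is below its maximum size.
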(event EventTick
  (params (DeltaSeconds :type Float%20%28single-precision%29))
  (CallFunction|SpawnResultItem 195453)
  (CallFunction|SpawnResultItem 195454)
  (CallFunction|SpawnResultItem 195455))

(event EventBeginPlay)

(event Collision|EventActorBeginOverlap
  (params (OtherActor :type Actor%20Object%20Reference)))

(fn ConstructionScript
  (|CallParentFunction))

(fn SpawnResultItem
  (params (templateID :type Integer))
  (Variables|Default|SetTemplateID%20to%20Spawn templateID)
  (if (< (Class|ItemInventory|GetPopulatedItemCount (Variables|Default|GetPlaceableInventory) 0 -1) (Variables|/Script/ConanSandbox.ItemInventory|GetMaxItemCount (Variables|Default|GetPlaceableInventory)))
    _
    (else
      (Variables|Default|SetCurrentInventoryIndex 0)
      (if (!= (Class|ItemInventory|FindItembyTemplateID (Variables|Default|GetPlaceableInventory) (Variables|Default|GetTemplateID%20to%20Spawn) (Variables|Default|GetCurrentInventoryIndex)) -1) :!label _label
        (if (< (Class|GameItem|GetIntStat (Class|ItemInventory|GetItem (Variables|Default|GetPlaceableInventory) (Class|ItemInventory|FindItembyTemplateID (Variables|Default|GetPlaceableInventory) (Variables|Default|GetTemplateID%20to%20Spawn) (Variables|Default|GetCurrentInventoryIndex))) "StackSize") (Class|GameItem|GetIntStat (Class|ItemInventory|GetItem (Variables|Default|GetPlaceableInventory) (Class|ItemInventory|FindItembyTemplateID (Variables|Default|GetPlaceableInventory) (Variables|Default|GetTemplateID%20to%20Spawn) (Variables|Default|GetCurrentInventoryIndex))) "MaxStackSize"))
          _
          (else
            (Variables|Default|SetCurrentInventoryIndex (+ (Variables|Default|GetCurrentInventoryIndex) 1))
            (goto _label)))
        (else
          (return)))))
  (Class|ItemInventory|AddItemTemplate (Variables|Default|GetPlaceableInventory) (Variables|Default|GetTemplateID%20to%20Spawn) -1 1 false 1.0 -1.0)
  (return))