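; Barber dye station placeable that lets players holding a Barber Token open a color radial menu, presumably for dyeing.
; On activation it checks the interacting character's backpack for the token and shows a missing-item notification otherwise.
; With a token, the server calls ShowFColorRadial on the controller's Funcom_PC_Extension component, then runs the parent activation.
; The token is not consumed here.
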(event EventInteractableActivate
  (params (Component :type Primitive%20Component%20Object%20Reference) (Instigator :type Player%20Controller%20Object%20Reference) (HitIndex :type Integer))
  (bind _asfun_combat_player_controller (Utilities|Casting|CastToFunCombat_PlayerController Instigator))
  (bind _asconan_character (Utilities|Casting|CastToConanCharacter (Pawn|GetControlledPawn _asfun_combat_player_controller)))
  (bind _returnvalue (Class|ConanCharacter|GetBackpackInventory _asconan_character))
  (if (Class|ItemInventory|HasItembyTemplateID _returnvalue 195106 1)
    (if (Networking|IsServer)
      (bind _asfun_combat_player_controller_2 (Utilities|Casting|CastToFunCombat_PlayerController Instigator))
      (if (> (Utilities|Array|Length (Actor|GetComponentsByClass _asfun_combat_player_controller_2 "/Game/Mods/Immersive_Sexiles_Extensions/Funcom_PC_Extension.Funcom_PC_Extension_C")) 0)
        (Default|ShowFColorRadial (Utilities|Array|Get(acopy) (Actor|GetComponentsByClass _asfun_combat_player_controller_2 "/Game/Mods/Immersive_Sexiles_Extensions/Funcom_PC_Extension.Funcom_PC_Extension_C")))
        (|CallParentFunction Component Instigator HitIndex)))
    (else
      (Default|NotificationText _asfun_combat_player_controller "Missing Item: Barber Token" false))))

(fn ConstructionScript
  (|CallParentFunction))