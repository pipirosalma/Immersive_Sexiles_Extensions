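; Hairdresser dye station, built on the BPBSCSit sit behaviour, that opens a hair color radial menu when activated.
; Activation runs the sit logic only if player character 0, rather than the instigator's pawn, has item template 195106 in its backpack.
; On the server it then finds the Hair_PlayerController component on the instigating FunCombat_PlayerController and calls ShowColorRadial.
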(event EventInteractableActivate
  (params (Component :type Primitive%20Component%20Object%20Reference) (Instigator :type Player%20Controller%20Object%20Reference) (HitIndex :type Integer))
  (Utilities|Casting|CastToFunCombat_PlayerController Instigator)
  (bind _asconan_character (Utilities|Casting|CastToConanCharacter (Game|GetPlayerCharacter 0)))
  (bind _returnvalue (Class|ConanCharacter|GetBackpackInventory _asconan_character))
  (if (Class|ItemInventory|HasItembyTemplateID _returnvalue 195106 1)
    (Default|InteractableActivate (Variables|Default|GetBP_BSC_Sit) Component Instigator HitIndex)
    (if (Networking|IsServer)
      (bind _asfun_combat_player_controller (Utilities|Casting|CastToFunCombat_PlayerController Instigator))
      (if (> (Utilities|Array|Length (Actor|GetComponentsByClass _asfun_combat_player_controller "/Game/Mods/Immersive_Sexiles_Extensions/Hair_PlayerController.Hair_PlayerController_C")) 0)
        (Default|ShowColorRadial (Utilities|Array|Get(acopy) (Actor|GetComponentsByClass _asfun_combat_player_controller "/Game/Mods/Immersive_Sexiles_Extensions/Hair_PlayerController.Hair_PlayerController_C")))))))

(fn ConstructionScript
  (|CallParentFunction))