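; Mod controller that adds the mod's content to the game by merging its extension data tables into the base tables.
; ModDataTableOperations runs a series of MergeDataTables calls covering items, recipes, profession templates, spawns, loot, crafting station names, equipment variations, feats and emotes.
; Tier 3 and 4 misc loot extensions also merge into their Highlands variants.
; The event graph and construction script contain no logic.
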(event EventBeginPlay)

(event EventTick
  (params (DeltaSeconds :type Float%20%28single-precision%29)))

(fn ConstructionScript)

(fn ModDataTableOperations
  (Class|ModController|MergeDataTables "/Game/Items/ItemTable.ItemTable" "/Game/Mods/Immersive_Sexiles_Extensions/Data_Table/dt_Exentsion_IItems.dt_Exentsion_IItems")
  (Class|ModController|MergeDataTables "/Game/Items/Recipes/RecipesTable.RecipesTable" "/Game/Mods/Immersive_Sexiles_Extensions/Data_Table/dt_Extension_Recipes.dt_Extension_Recipes")
  (Class|ModController|MergeDataTables "/Game/Systems/SpawnTable/ProfessionTemplateDataTable.ProfessionTemplateDataTable" "/Game/Mods/Immersive_Sexiles_Extensions/Data_Table/dt_Extension_Profession_Template_Overwrites.dt_Extension_Profession_Template_Overwrites")
  (Class|ModController|MergeDataTables "/Game/Systems/SpawnTable/SpawnDataTable.SpawnDataTable" "/Game/Mods/Immersive_Sexiles_Extensions/Data_Table/dt_Extension_Spawn_Table.dt_Extension_Spawn_Table")
  (Class|ModController|MergeDataTables "/Game/Systems/Loot/TableSetup/W_T2MiscLoot.W_T2MiscLoot" "/Game/Mods/Immersive_Sexiles_Extensions/Data_Table/dt_Extension_W_Misc_Loot_T2.dt_Extension_W_Misc_Loot_T2")
  (Class|ModController|MergeDataTables "/Game/Systems/Loot/TableSetup/W_T3MiscLoot.W_T3MiscLoot" "/Game/Mods/Immersive_Sexiles_Extensions/Data_Table/dt_Extension_W_Misc_Loot_T3.dt_Extension_W_Misc_Loot_T3")
  (Class|ModController|MergeDataTables "/Game/Systems/Loot/TableSetup/W_T4MiscLoot.W_T4MiscLoot" "/Game/Mods/Immersive_Sexiles_Extensions/Data_Table/dt_Extension_W_Misc_Loot_T4.dt_Extension_W_Misc_Loot_T4")
  (Class|ModController|MergeDataTables "/Game/Systems/Loot/TableSetup/W_T3MiscLoot_Highlands.W_T3MiscLoot_Highlands" "/Game/Mods/Immersive_Sexiles_Extensions/Data_Table/dt_Extension_W_Misc_Loot_T3.dt_Extension_W_Misc_Loot_T3")
  (Class|ModController|MergeDataTables "/Game/Systems/Loot/TableSetup/W_T4MiscLoot_Highlands.W_T4MiscLoot_Highlands" "/Game/Mods/Immersive_Sexiles_Extensions/Data_Table/dt_Extension_W_Misc_Loot_T4.dt_Extension_W_Misc_Loot_T4")
  (Class|ModController|MergeDataTables "/Game/Items/Crafting/CraftingStationNameTable.CraftingStationNameTable" "/Game/Mods/Immersive_Sexiles_Extensions/Data_Table/dt_Extension_Crafting_Name.dt_Extension_Crafting_Name")
  (Class|ModController|MergeDataTables "/Game/Items/EquipmentVariationTable.EquipmentVariationTable" "/Game/Mods/Immersive_Sexiles_Extensions/Data_Table/dt_Extensions_Equip_Var.dt_Extensions_Equip_Var")
  (Class|ModController|MergeDataTables "/Game/Items/Feats/FeatTable.FeatTable" "/Game/Mods/Immersive_Sexiles_Extensions/Data_Table/dt_Extension_Feat_Table.dt_Extension_Feat_Table")
  (Class|ModController|MergeDataTables "/Game/Characters/Emotes/EmotesDataTable.EmotesDataTable" "/Game/Mods/Immersive_Sexiles_Extensions/Data_Table/dt_New_Emotes.dt_New_Emotes"))