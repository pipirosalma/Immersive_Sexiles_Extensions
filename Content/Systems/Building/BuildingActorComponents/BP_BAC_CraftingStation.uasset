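; Building actor component that makes its owning actor an interactable crafting station in Conan.
; Activation toggles the crafting GUI through the pawn's interacting actor, and losing selection while open closes it.
; For buildables, an ownership check picks between two GUI modules, with non-buildables getting the owner's version.
; BeginPlay loads saved inventory by each persistence component's unique ID and processes it onto the owner.
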(event EventInteractableActivate
  (params (Component :type Primitive%20Component%20Object%20Reference) (Instigator :type Player%20Controller%20Object%20Reference) (HitIndex :type Integer))
  (bind _returnvalue (Pawn|GetControlledPawn Instigator))
  (bind _returnvalue_2 (Components|GetOwner))
  (bind _asconan_character (Utilities|Casting|CastToConanCharacter _returnvalue))
  (if (Variables|Default|GetIsOpen)
    (Variables|Default|SetIsOpen false)
    (Class|ConanCharacter|SetInteractingActor _asconan_character 0 "None")
    (else
      (Variables|Default|SetIsOpen true)
      (bind _asbuildable_base (Utilities|Casting|CastToBuildableBase _returnvalue_2)
        (:then
          (if (Class|BuildableBase|IsOwner _asbuildable_base _returnvalue false)
            (Class|ConanCharacter|SetInteractingActor _asconan_character _returnvalue_2 "CraftingGUI" :!label _label)
            (else
              (Class|ConanCharacter|SetInteractingActor _asconan_character _returnvalue_2 "CraftingGUI_2"))))
        (:CastFailed
          (goto _label))))))

(event EventBeginPlay
  (for _array_element (Actor|GetComponentsByClass (Components|GetOwner) "/Script/ConanSandbox.ConanBuildingPersistenceComponent")
    (bind _result (|LoadInventory (Class|PersistenceComponent|GetUniqueID _array_element))
      (:OnSuccess
        (Class|LoadInventoryCallProxy|ProcessInventoryData (Components|GetOwner) _result)))))

(event EventInteractableSelectionChanged
  (params (IsSelected :type Boolean) (Instigator :type Player%20Controller%20Object%20Reference) (InstanceIndex :type Integer))
  (if (and (not IsSelected) (Variables|Default|GetIsOpen))
    (Variables|Default|SetIsOpen false)
    (Class|ConanCharacter|SetInteractingActor (.AsConan%20Character (Utilities|Casting|CastToConanCharacter (Pawn|GetControlledPawn (stale EventInteractableActivate Instigator)))) 0 "None")))