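; Placeable religious altar that logs a VenerateGods journey event on interaction and spawns a protective-style dome when its dome recipe is crafted.
; The crafting queue signal replaces any existing dome with a new persistent actor, tracked by unique ID and removed when the altar is destroyed.
; The construction script tints the tier 3 beam through a dynamic material.
; The recipe-start notification is unfinished and unbound, and the craftability check always passes.
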(event Custom|On%20Recipe%20Started
  (params (index :type Integer) (item :type Game%20Item%20Object%20Reference) (srcInventory :type Item%20Inventory%20Object%20Reference) (srcIndex :type Integer))
  (bind _templateid (Variables|/Script/ConanSandbox.GameItem|GetTemplateID item))
  ;[1 0 0] DO STUFF HERE TO MAKE THE ALTAR SPAWN A MAP MARKER AND A BEAM - WIP
  (if (Utilities|Array|ContainsItem (Variables|Default|GetNotify%20Altar%20Upgrade%20Recipe%20IDs) _templateid)
    (bind _name (CallFunction|GetNamefromTemplateID _templateid))
    (Development|PrintString (Utilities|String|ToString(Text) (Utilities|Text|FormatText "A new {recipename} has started!" _name)))))

(event Custom|On%20Recipe%20Crafted
  (params (recipeItem :type Recipe%20Item%20Object%20Reference))
  ;[1 1 1] On Recipe Crafted
  (if (== (Variables|/Script/ConanSandbox.GameItem|GetTemplateID recipeItem) (Variables|Default|GetDome%20Recipe%20ID))
    (CallFunction|DestroyDome)
    (bind _returnvalue (Game|SpawnActorfromClass (Variables|Default|GetDome%20Class) (Math|Transform|MakeTransform (Transformation|GetActorLocation self)) "AlwaysSpawn" 0 0))
    (bind _returnvalue_2 (Class|UniqueID|GenerateUniqueID))
    (bind _output_get (Variables|Default|SetDome%20Unique%20ID _returnvalue_2))
    (Class|DreamworldBlueprints|SetUniqueID _returnvalue _output_get)
    (Class|PersistenceComponent|SetDirty (Variables|/Game/Systems/Avatar/BP_AvatarDome.BP_AvatarDome_C|GetActorPersistence _returnvalue) true 5.0)))

(event EventInteractableActivate
  (params (Component :type Primitive%20Component%20Object%20Reference) (Instigator :type Player%20Controller%20Object%20Reference) (HitIndex :type Integer))
  (bind _returnvalue (Pawn|GetControlledPawn Instigator))
  (|CallParentFunction Component Instigator HitIndex)
  (Class|ExilesJourneyComponent|AddJourneyEvent (Actor|GetComponentbyClass _returnvalue "/Game/Systems/Progression/BP_AC_ExilesJourney.BP_AC_ExilesJourney_C") "VenerateGods" (Transformation|GetActorLocation _returnvalue)))

(event EventDestroyed
  (CallFunction|DestroyDome))

(event Game|Damage|EventAnyDamage
  (params (Damage :type Float%20%28single-precision%29) (DamageType :type Damage%20Type%20Object%20Reference) (InstigatedBy :type Controller%20Object%20Reference) (DamageCauser :type Actor%20Object%20Reference) (DamageEventID :type Integer))
  (Development|PrintString (Utilities|String|ToString(Text) (Utilities|Text|FormatText "{target} got hit by {hitter} for {damage}({damagetype})" (Utilities|Text|ToText(String) (Utilities|GetDisplayName self)) (Utilities|Text|ToText(String) (Utilities|GetDisplayName DamageCauser)) (Utilities|Text|ToText(Float) Damage "HalfToEven") (Utilities|Text|ToText(String) (Utilities|GetDisplayName DamageType))))))

(event EventBeginPlay
  (bind _craftingqueue (Variables|Default|GetCraftingQueue))
  (Utilities|FlowControl|Sequence
    (:then_0
      (EventDispatchers|BindEventtoSignalRecipeCrafted _craftingqueue (delegate Custom|On%20Recipe%20Crafted))
      (Variables|/Script/ConanSandbox.CraftingQueue|SetDelegateCanRecipeBeCrafted _craftingqueue (EventDispatchers|CreateEvent :!event SlotCanRecipebeCrafted))
      (|CallParentFunction))))

(fn ConstructionScript
  (bind _tier3beameffect (Variables|Default|GetTier3BeamEffect))
  (Utilities|IsValid+Branch _tier3beameffect (> (Rendering|Material|GetNumMaterials _tier3beameffect) 0)
    (:True
      (bind _returnvalue (Rendering|Material|CreateDynamicMaterialInstance _tier3beameffect 0 (Rendering|Material|GetMaterial _tier3beameffect 0) :!class /Script/Engine.PrimitiveComponent))
      (Rendering|Material|SetVectorParameterValue _returnvalue "colorglow" (Variables|Default|GetTier%203%20Beam%20Color) :!class /Script/Engine.MaterialInstanceDynamic))
    (:False%20or%20Invalid
      _))
  (|CallParentFunction))

(fn SlotCanRecipebeCrafted
  (params (CraftingQueue :type Crafting%20Queue%20Object%20Reference) (Recipe :type Recipe%20Item%20Object%20Reference))
  (return true))

(fn DestroyDome
  (bind _asbase_game_mode_interface (Utilities|Casting|CastToBaseGameModeInterface (Game|GetGameMode)))
  (bind _actor (Default|GetActorbyUniqueIDInterface _asbase_game_mode_interface (Variables|Default|GetDome%20Unique%20ID)))
  (Utilities|IsValid _actor
    (:Is%20Valid
      (Actor|DestroyActor _actor))))