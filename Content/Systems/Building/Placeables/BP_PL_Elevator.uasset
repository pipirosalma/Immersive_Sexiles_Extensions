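; Placeable elevator whose cage travels between its top and the ground below, toggled by two pull chains or a lever.
; A timeline scaled to travel distance drives cage motion, sway and cog, with sounds and an arrival camera shake.
; The server box-traces the landing once and stores it, replicating it to position the pad and claimed area.
; Placement rejects overlaps or insufficient drop; clients request playback-position sync on BeginPlay.
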(event Custom|SetLandingPosition
  (bind _claimedareabox (Variables|Default|GetClaimedAreaBox))
  (bind _startloc (Variables|Default|GetStartLoc))
  (bind _endlocation (Variables|Default|GetEndLocation))
  (bind _returnvalue (Transformation|GetWorldTransform _startloc))
  (bind _returnvalue_2 (Math|Transform|InverseTransformLocation _returnvalue _endlocation))
  (bind _returnvalue_3 (/ (.z _returnvalue_2) 2.0))
  ;[1 1 1] Set the landing pad location. Being replicated when End Location gets relevancy.
  (Transformation|SetRelativeLocation (Variables|Default|GetLandingpad) (Math|Vector|MakeVector 0.0 0.0 (.z _returnvalue_2)) false false)
  (Transformation|SetRelativeLocation _claimedareabox (Math|Vector|MakeVector 0.0 0.0 _returnvalue_3) false false)
  (Components|Box|SetBoxExtent _claimedareabox (Math|Vector|MakeVector 1e+02 1e+02 (Math|Float|Absolute(Float) _returnvalue_3)) true)
  (Utilities|FlowControl|Delay 1.0)
  (Rendering|SetVisibility (Variables|Default|GetCable) true false))

(event Custom|DoMovement
  (params (GoingUp :type Boolean) (TimelineSpeed :type Float%20%28single-precision%29))
  (CallFunction|CheckMainSound)
  (Components|Timeline|SetPlayRate (Variables|Default|GetTimeline_0) TimelineSpeed)
  (if GoingUp
    (bind (_direction _locationmovement _rotationmovement) (Timeline|Timeline_0 Reverse)
      (:Update
        (Transformation|SetRelativeRotation (Variables|Default|GetStaticMesh) (Math|Rotator|CombineRotators (Variables|Default|GetDefCageRot) (Math|Rotator|MakeRotator (* (.X (Math|Vector|BreakVector _rotationmovement)) 0.5) (* (.Y (Math|Vector|BreakVector _rotationmovement)) 0.5) (* (.Z (Math|Vector|BreakVector _rotationmovement)) 1.0))) false false)
        (Transformation|SetRelativeLocation (Variables|Default|GetStaticMesh) (+ (* (Math|Transform|InverseTransformLocation (Transformation|GetWorldTransform (Variables|Default|GetStartLoc)) (+ (Variables|Default|GetEndLocation) "0, 0,0.000000")) _locationmovement) (Variables|Default|GetDefCageLoc)) false false)
        (Transformation|AddRelativeRotation (Variables|Default|GetCog2) (* (select (Variables|Default|GetGoingUp) "0.000000,0,-16.000000" "0.000000,0,16.000000") _locationmovement) false false)
        (if (Networking|IsServer)
          (Variables|Default|SetPlaybackPosition _locationmovement)))
      (:Finished
        (CallFunction|StopMainSound)
        ;[1 1 1] Camera Shake
        (Camera|PlayWorldCameraShake "/Game/Systems/Combat/CameraShake/BP_CameraShakeDefault.BP_CameraShakeDefault_C" (+ (Transformation|GetWorldLocation (Variables|Default|GetCage)) "0, 0,128.000000") 0.0 256.0)))
    (else
      (Timeline|Timeline_0 Play))))

(event Custom|PlayLeverSound
  ;[1 1 1] Sounds
  (if (not (Networking|IsDedicatedServer))
    (Class|ConanAudioComponent|LoadandPlay (Variables|Default|GetLeverSound) 0.0)))

(event Custom|StopMainSound
  ;[1 1 1] Sounds
  (if (not (Networking|IsDedicatedServer))
    (Class|ConanAudioComponent|Stop (Variables|Default|GetElevatorSound))
    (Class|ConanAudioComponent|LoadandPlay (Variables|Default|GetSettleSoundElevator) 0.0)
    (Class|ConanAudioComponent|LoadandPlay (Variables|Default|GetRopeCogSettleSound) 0.0)))

(event Custom|ChainMovementEvent
  (params (ComponentToMove :type Primitive%20Component%20Object%20Reference) (DefaultLoc :type Vector) (ChainNumber :type Integer))
  (CallFunction|PlayChainSound ChainNumber)
  (bind _chainm (Timeline|ChainMovement PlayFromStart)
    (:Update
      (Transformation|SetRelativeLocation ComponentToMove (+ DefaultLoc _chainm) false false))))

(event Custom|CheckMainSound
  ;[1 1 1] Sounds
  (if (not (Networking|IsDedicatedServer))
    (if (not (Class|ConanAudioComponent|IsPlaying (Variables|Default|GetRopeCogSound)))
      (Class|ConanAudioComponent|LoadandFadein (Variables|Default|GetElevatorSound) 1.0 1.0 0.0))))

(event Custom|FindGround
  (bind _startloc (Variables|Default|GetStartLoc))
  (bind _returnvalue (Transformation|GetWorldLocation _startloc))
  ;[1 1 1] We find the landing pos on creation, then store it. Otherwise trace will go through buildings before they load.
  (Variables|Default|SetFoundGround true)
  (bind _outhit (Collision|BoxTraceByChannel _returnvalue (- _returnvalue (Variables|Default|GetMaxElevatorDistance)) "96.000000,96.000000,1.000000" (Transformation|GetWorldRotation (Variables|Default|GetStaticMesh)) "TraceTypeQuery1" false 0 "None"))
  (bind _output_get (Variables|Default|SetElevatorTraceResult _outhit))
  (Variables|Default|SetEndLocation (.Location (Collision|BreakHitResult _output_get)))
  (CallFunction|SetLandingPosition))

(event Custom|LeverMovement
  (CallFunction|PlayLeverSound)
  (bind _newtrack_1 (Timeline|LeverTimeline PlayFromStart)
    (:Update
      (Transformation|SetRelativeLocation (Variables|Default|GetLever) (+ (* _newtrack_1 (select (Variables|Default|GetGoingUp) -1.0 1.0)) (Variables|Default|GetLeverDefLoc)) false false))))

(event Custom|PlayChainSound
  (params (ChainNumber :type Integer))
  ;[1 1 1] Sounds
  (if (not (Networking|IsDedicatedServer))
    (Class|ConanAudioComponent|LoadandPlay (Utilities|Select :Index ChainNumber :Option%200 (Variables|Default|GetChain0Sound) :Option%201 (Variables|Default|GetChain1Sound)) 0.0)))

(event EventInteractableActivate
  (params (Component :type Primitive%20Component%20Object%20Reference) (Instigator :type Player%20Controller%20Object%20Reference) (HitIndex :type Integer))
  (if (== Component (Variables|Default|GetBox))
    (CallFunction|ChainMovementEvent (Variables|Default|GetChain0) (Variables|Default|GetChain0DefRelLoc))
    (Utilities|FlowControl|FlipFlop :!label _label
      (:A
        (Variables|Default|SetGoingUp false))
      (:B
        (Variables|Default|SetGoingUp true)))
    (bind _output_get (Variables|Default|SetTimeLineSpeed (/ (Variables|Default|GetUnitsPerSecond) (Math|Vector|VectorLength (- (Transformation|GetWorldLocation (Variables|Default|GetStartLoc)) (Variables|Default|GetEndLocation))))))
    (CallFunction|DoMovement (Variables|Default|GetGoingUp) _output_get)
    (elif (== Component (Variables|Default|GetBox1))
      (CallFunction|ChainMovementEvent (Variables|Default|GetChain1) (Variables|Default|GetChain1DefRelLoc) 1)
      (goto _label)
      (elif (== Component (Variables|Default|GetBox2))
        (CallFunction|LeverMovement)
        (goto _label)))))

(event EventClientRequestSynconServer
  (if (Networking|IsServer)
    (Variables|Default|SetRepPlaybackPosition (Variables|Default|GetPlaybackPosition))))

(event EventBeginPlay
  (if (Networking|IsServer)
    (if (Variables|Default|GetFoundGround)
      (CallFunction|SetLandingPosition)
      (else
        (CallFunction|FindGround)))
    (else
      (bind _asfun_combat_player_controller (Utilities|Casting|CastToFunCombat_PlayerController (Game|GetPlayerController 0)))
      (Default|SyncActoronServer _asfun_combat_player_controller self))))

(fn ConstructionScript
  (bind _staticmesh (Variables|Default|GetStaticMesh))
  (|CallParentFunction)
  (Variables|Default|SetDefCageLoc (Variables|/Script/Engine.SceneComponent|GetRelativeLocation _staticmesh))
  (Variables|Default|SetDefCageRot (Variables|/Script/Engine.SceneComponent|GetRelativeRotation _staticmesh))
  (Variables|Default|SetChain0DefRelLoc (Variables|/Script/Engine.SceneComponent|GetRelativeLocation (Variables|Default|GetChain0)))
  (Variables|Default|SetChain1DefRelLoc (Variables|/Script/Engine.SceneComponent|GetRelativeLocation (Variables|Default|GetChain1)))
  (Variables|Default|SetLeverDefLoc (Variables|/Script/Engine.SceneComponent|GetRelativeLocation (Variables|Default|GetLever))))

(fn OnRepEndLocation
  (CallFunction|SetLandingPosition))

(fn OnRepRepPlaybackPosition
  (Components|Timeline|SetPlaybackPosition (Variables|Default|GetTimeline_0) (Variables|Default|GetRepPlaybackPosition) false true))

(fn CanbePlaced
  (params (AttachTo :type Buildable%20Base%20Object%20Reference) (InstanceIndex :type Integer))
  (bind _startloc (Variables|Default|GetStartLoc))
  (bind _returnvalue (Transformation|GetWorldLocation _startloc))
  (bind (_failedmessage _returnvalue_2) (|CallParentFunction AttachTo InstanceIndex))
  (if (> (Utilities|Array|Length (Class|FuncomGenericLibrary|GetOverlappingActorsasHitResults (Variables|Default|GetPlacementCheckBox) "/Game/Systems/Building/BP_BuildingBase.BP_BuildingBase_C")) 0)
    (return (Utilities|String|ToString(Text) (Variables|Default|GetError_Overlapping)) "Fail_Overlaps")
    (else
      (bind (_outhit _returnvalue_3) (Collision|BoxTraceByChannel _returnvalue (- _returnvalue (Variables|Default|GetMaxElevatorDistance)) "96.000000,96.000000,1.000000" (Transformation|GetWorldRotation (Variables|Default|GetStaticMesh)) "TraceTypeQuery1" false 0 "None"))
      (if _returnvalue_3
        (if (> (Math|Vector|VectorLength (- _returnvalue (.Location (Collision|BreakHitResult _outhit)))) 2e+02)
          (return _failedmessage _returnvalue_2)
          (else
            _)))
      (return (Variables|Default|GetError_UnableToFindEndLoc) "Fail"))))

(fn ProvidesShelter
  (return true))