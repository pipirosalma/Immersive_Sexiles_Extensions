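; Placeable thrall converter crafting station (the wheel, per its journey event) that turns captured NPCs into thrall items.
; On interaction, an owner dragging a thrall starts thrallifying the prisoner and logs a journey step.
; ConverThrall spawns an item from the NPC and its character layout into the placeable inventory.
; NPCs without a ThrallID convert only if the profession table's Default row exists, otherwise an error is logged.
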(event EventConverThrall
  (params (ThrallActor :type Actor%20Object%20Reference))
  (bind _asconan_character (Utilities|Casting|CastToConanCharacter ThrallActor))
  (bind _asi_has_character_layout_interface (Utilities|Casting|CastToI_HasCharacterLayoutInterface ThrallActor))
  (bind _character_layout (Default|GetCharacterLayout _asi_has_character_layout_interface))
  (if (!= (Class|ConanCharacter|GetIntStat _asconan_character "ThrallID" "Base") 0)
    (bind _returnvalue (Class|GameItemSpawner|SpawnThrallItem "/Script/ConanSandbox.ThrallItem" _asconan_character _character_layout))
    (Class|ItemInventory|AddItem (Variables|Default|GetPlaceableInventory) _returnvalue -1 0 -1)
    (else
      (bind _returnvalue_2 (Utilities|GetDataTableRow "/Game/Systems/SpawnTable/ProfessionTemplateDataTable.ProfessionTemplateDataTable" "Default")
        (:then
          (bind _returnvalue_3 (Class|GameItemSpawner|SpawnThrallItem "/Script/ConanSandbox.ThrallItem" _asconan_character _character_layout))
          (Class|ItemInventory|AddItem (Variables|Default|GetPlaceableInventory) _returnvalue_3 -1 0 -1))
        (:RowNotFound
          (Class|LoggerLibrary|DWLogString "Could not find Default fallback for ProfessionTemplateDataTable." "Thrall" "INFOL_DATAERROR"))))))

(event EventBeginPlay
  (|CallParentFunction))

(event Collision|EventActorBeginOverlap
  (params (OtherActor :type Actor%20Object%20Reference)))

(event EventTick
  (params (DeltaSeconds :type Float%20%28single-precision%29)))

(event EventInteractableActivate
  (params (Component :type Primitive%20Component%20Object%20Reference) (Instigator :type Player%20Controller%20Object%20Reference) (HitIndex :type Integer))
  (bind _returnvalue (Pawn|GetControlledPawn Instigator))
  (bind _returnvalue_2 (Pawn|GetControlledPawn Instigator))
  (bind _asthrall_owner_interface (Utilities|Casting|CastToThrallOwnerInterface _returnvalue))
  (bind _returnvalue_3 (Class|ThrallOwnerInterface|IsDraggingThrall _asthrall_owner_interface))
  (if _returnvalue_3
    (if (Class|BuildableBase|IsOwner _returnvalue false)
      (Class|ThrallOwnerInterface|StartThrallifyingPrisoner _asthrall_owner_interface self)
      (Class|ExilesJourneyComponent|AddJourneyEvent (Actor|GetComponentbyClass _returnvalue_2 "/Game/Systems/Progression/BP_AC_ExilesJourney.BP_AC_ExilesJourney_C") "NPCToWheel" (Transformation|GetActorLocation _returnvalue_2))))
  (|CallParentFunction 0 Instigator HitIndex))

(fn ConstructionScript
  (|CallParentFunction))

(fn GetResourceInventory
  (return (Variables|Default|GetPlaceableInventory)))

(fn InteractableMenuDisabled
  (return false))

(fn InteractableDefaultAction
  (return "Interact" "/Game/UI/Textures/GUIs/MainRadialMenu/T_MainRadialMenuIconInteract.T_MainRadialMenuIconInteract"))

(fn GetArtisanThrallInventory
  (return (Variables|Default|GetThrallInventory)))